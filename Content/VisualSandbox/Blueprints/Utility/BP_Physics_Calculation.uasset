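; BP_Physics_Calculation is a utility Blueprint of physics math helpers for drag force and PID control.
; CalculateDragForce applies the quadratic drag equation to air density, drag coefficient, frontal area and speed.
; ComputePID sums proportional, integral and derivative terms into a force, returning it with gains and error state in a new FPIDData for the next call.
; The returned AccumulatedError holds the error's rate of change instead of the running integral.
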(fn `Calculate Drag Force`
  (params (`Air Density` :type "Float (double-precision)" :default 0.000122) (`Drag Coef` :type "Float (double-precision)" :default 0.5) (`Frontal Area` :type "Float (double-precision)" :default 400.0) (`Object Speed` :type "Float (double-precision)"))
  (returns (ReturnValue :type "Float (double-precision)"))
  (return (* 0.5 `Air Density` `Drag Coef` `Frontal Area` (`KismetMathLibrary.Square` `Object Speed`))))

(fn `Compute PID`
  (params (`PID Values` :type "/Game/VisualSandbox/Blueprints/Structures/FPID_Data Structure") (Error :type "Float (double-precision)") (`Delta Time` :type "Float (double-precision)"))
  (returns (`PID Update` :type "/Game/VisualSandbox/Blueprints/Structures/FPID_Data Structure"))
  (locals (P :type "Float (double-precision)") (I :type "Float (double-precision)") (D :type "Float (double-precision)"))
  (bind (_pid_values_kp _pid_values_ki _pid_values_kd _pid_values_accumulatederror _pid_values_previouseerror) (break `/Game/VisualSandbox/Blueprints/Structures/FPID_Data` (`local.PID Values`)))
  (bind (_pid_values_kp_2 _pid_values_ki_2 _pid_values_kd_2 _pid_values_accumulatederror_2) (break `/Game/VisualSandbox/Blueprints/Structures/FPID_Data` (`local.PID Values`)))
  (bind _pid_values_kp_3 (break `/Game/VisualSandbox/Blueprints/Structures/FPID_Data` (`local.PID Values`)))
  (bind (_pid_values_kp_4 _pid_values_ki_3 _pid_values_kd_3) (break `/Game/VisualSandbox/Blueprints/Structures/FPID_Data` (`local.PID Values`)))
  (bind (_pid_values_kp_5 _pid_values_ki_4) (break `/Game/VisualSandbox/Blueprints/Structures/FPID_Data` (`local.PID Values`)))
  (bind (_pid_values_kp_6 _pid_values_ki_5 _pid_values_kd_4) (break `/Game/VisualSandbox/Blueprints/Structures/FPID_Data` (`local.PID Values`)))
  (bind (_pid_values_kp_7 _pid_values_ki_6 _pid_values_kd_5 _pid_values_accumulatederror_3 _pid_values_previouseerror_2) (break `/Game/VisualSandbox/Blueprints/Structures/FPID_Data` (`local.PID Values`)))
  (set `local.P` (* (`local.Error`) _pid_values_kp_3))
  (set `local.I` (* (+ _pid_values_accumulatederror_2 (* (`local.Error`) (`local.Delta Time`))) _pid_values_ki_4))
  (set `local.D` (* (/ (- (`local.Error`) _pid_values_previouseerror_2) (`local.Delta Time`)) _pid_values_kd_4))
  (return (make `/Game/VisualSandbox/Blueprints/Structures/FPID_Data` _pid_values_kp_4 _pid_values_ki_3 _pid_values_kd_3 (/ (- (`local.Error`) _pid_values_previouseerror) (`local.Delta Time`)) (`local.Error`) (+ (`local.P`) (`local.I`) (`local.D`)))))