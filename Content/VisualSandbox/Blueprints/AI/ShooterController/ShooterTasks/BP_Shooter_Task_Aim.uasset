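; Behavior tree task that makes a shooter AI aim at the actor stored in its Target blackboard value.
; On execute it runs the parent logic, sets controller focus on the target and tells the shooter pawn to start aiming, with no finish call of its own.
; On abort it stops aiming, clears focus and finishes the abort.
; A helper function returns the pawn's distance to the target.
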(event `self.ReceiveExecuteAI`
  (params (OwnerController :type "AIController Object Reference") (ControlledPawn :type "Pawn Object Reference"))
  (`parent.ReceiveExecuteAI` OwnerController ControlledPawn)
  (set `self.Target Actor` (`BTFunctionLibrary.GetBlackboardValueAsActor` (`self.Target`)))
  (`AIController.K2_SetFocus` (`self.ShooterController`) (`self.Target Actor`))
  (bind _shooterpawn (`self.ShooterPawn`)
    (:`then`
      (`/Game/VisualSandbox/Blueprints/Characters/BP_ShooterCharacter.Start Aiming` _shooterpawn true))
    (:`else`)))

(event `self.ReceiveAbortAI`
  (params (OwnerController :type "AIController Object Reference") (ControlledPawn :type "Pawn Object Reference"))
  (`|ExecutionSequence`
    (:`then_0`
      (bind _shooterpawn (`self.ShooterPawn`)
        (:`then`
          (`/Game/VisualSandbox/Blueprints/Characters/BP_ShooterCharacter.Start Aiming` _shooterpawn false))
        (:`else`)))
    (:`then_1`
      (`AIController.K2_ClearFocus` (`self.ShooterController`))
      (`self.FinishAbort`))))

(fn `Get Taget Distance`
  (returns (ReturnValue :type "Float (single-precision)"))
  (return (`Actor.GetDistanceTo` (`self.ShooterPawn`) (`self.Target Actor`))))