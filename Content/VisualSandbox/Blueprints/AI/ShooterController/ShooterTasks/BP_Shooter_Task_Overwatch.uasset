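; Behavior tree task for the shooter AI that makes a bot turn to watch a random direction.
; On execute it runs the parent setup, clears the controller's focus and picks a random yaw with level pitch and roll.
; Each tick it passes that rotation to the shooter controller with lag, and finishes successfully once the controller's rotation update returns true.
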(event `self.ReceiveExecuteAI`
  (params (OwnerController :type "AIController Object Reference") (ControlledPawn :type "Pawn Object Reference"))
  (`parent.ReceiveExecuteAI` OwnerController ControlledPawn)
  (`AIController.K2_ClearFocus` (`self.ShooterController`))
  (set `self.Desired Control Rotation` (`KismetMathLibrary.MakeRotator` 0.0 0.0 (`KismetMathLibrary.RandomFloatInRange` 0.0 360.0))))

(event `self.ReceiveTickAI`
  (params (OwnerController :type "AIController Object Reference") (ControlledPawn :type "Pawn Object Reference") (DeltaSeconds :type "Float (single-precision)"))
  ; Update Bot Control Rotation
  (bind _successful (`/Game/VisualSandbox/Blueprints/AI/Common/BP_BotController.Set Bot Control Rotation` (`self.ShooterController`) (`self.Desired Control Rotation`) 1.0))
  (if _successful
    (`self.FinishExecute` true)))