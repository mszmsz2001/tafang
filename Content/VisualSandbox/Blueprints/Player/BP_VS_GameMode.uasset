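; Game mode for the Visual Sandbox player setup, handling bullet time, respawning, level restart and quitting.
; Bullet time plays or reverses a timeline that blends global time dilation and matches slow-motion sound pitch to it through a sound mix override.
; Respawn spawns a default pawn at the respawn point nearest the controlled pawn, then possesses it and notifies the controller.
; Main-character getter and pause setter are empty stubs.
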(event `/Game/VisualSandbox/Blueprints/Interfaces/BPI_Game.Activate Bullet Time`
  ; Activate and Deactivate Bullet Time mode
  (set `self.Is Bullet Time Ativated` true)
  (`GameplayStatics.PlaySound2D` "/Game/VisualSandbox/Audio/Cue/Misc/Slomo_Start_Cue.Slomo_Start_Cue" 1.0 1.0 0.0 null null)
  (bind (_direction _interpolation) (`Timeline|Smooth bullet time transition` :!label _label)
    (:`Update`
      (`GameplayStatics.SetGlobalTimeDilation` (`KismetMathLibrary.Lerp` 1.0 (`self.Bullet Time Speed`) _interpolation)) ; slow down time
      (`GameplayStatics.SetSoundMixClassOverride` "/Game/VisualSandbox/Audio/Mix/SCM_SlomoMix.SCM_SlomoMix" "/Game/VisualSandbox/Audio/Mix/SC_Slomo.SC_Slomo" 1.0 (`GameplayStatics.GetGlobalTimeDilation`) :!pinned true) ; Pitch down sound effects
      (`GameplayStatics.PushSoundMixModifier` "/Game/VisualSandbox/Audio/Mix/SCM_SlomoMix.SCM_SlomoMix"))))

(event `/Game/VisualSandbox/Blueprints/Interfaces/BPI_Game.Deactivate Bullet Time`
  ; Activate and Deactivate Bullet Time mode
  (set `self.Is Bullet Time Ativated` false)
  (`GameplayStatics.PlaySound2D` "/Game/VisualSandbox/Audio/Cue/Misc/Slomo_Stop_Cue.Slomo_Stop_Cue" 1.0 1.0 0.0 null null)
  (goto _label :!via `Reverse`))

(event `/Game/VisualSandbox/Blueprints/Interfaces/BPI_Game.Toggle Bullet Time`
  ; Activate and Deactivate Bullet Time mode
  (if (`self.Is Bullet Time Ativated`)
    (`self.Deactivate Bullet Time`)
    (else
      (`self.Activate Bullet Time`))))

(event `self.ReceiveBeginPlay`
  ; Begin Play
  (`WidgetBlueprintLibrary.SetInputMode_GameOnly` (`GameplayStatics.GetPlayerController` 0))
  (`GameplayStatics.SetSoundMixClassOverride` "/Game/VisualSandbox/Audio/Mix/SCM_SlomoMix.SCM_SlomoMix" "/Game/VisualSandbox/Audio/Mix/SC_Slomo.SC_Slomo" 1.0 (`GameplayStatics.GetGlobalTimeDilation`) :!pinned true) ; Reset bullet time pitch sound
  (`GameplayStatics.PushSoundMixModifier` "/Game/VisualSandbox/Audio/Mix/SCM_SlomoMix.SCM_SlomoMix"))

(event `/Game/VisualSandbox/Blueprints/Interfaces/BPI_Game.Quit Game`
  ; Quit the game by executing the "Quit" console commnad
  (`KismetSystemLibrary.ExecuteConsoleCommand` "Quit" null))

(event `/Game/VisualSandbox/Blueprints/Interfaces/BPI_Game.Respawn`
  (params (`Player Controller` :type "PlayerController Object Reference"))
  ; Respawn player
  (`self.Respawn Player` `Player Controller`))

(event `/Game/VisualSandbox/Blueprints/Interfaces/BPI_Game.Restart Game`
  ; Restart game by reloading the current map
  (bind _returnvalue (`GameplayStatics.GetCurrentLevelName` true))
  (`GameplayStatics.OpenLevel` (`KismetStringLibrary.Conv_StringToName` _returnvalue)))

(fn `Get Main Character`
  (returns (`Return Main Character` :type "Pawn Object Reference"))
  (return null))

(fn `Respawn Player`
  (params (PC :type "PlayerController Object Reference"))
  (locals (`Respawn Points Found` :type "Array of Actor Object Reference") (SpawnedPawn :type "Pawn Object Reference"))
  (bind _returnvalue (`self.GetTransform` (`/Game/VisualSandbox/Blueprints/Utility/BP_UsefulFunctions.Find Nearest Actor` (`local.Respawn Points Found`) (`Controller.K2_GetPawn` (`local.PC`)))))
  (`|ExecutionSequence`
    (:`then_0`
      ; Find all respawn points
      (bind _outactors (`GameplayStatics.GetAllActorsOfClass` "/Game/VisualSandbox/Blueprints/Systems/BP_RespawnPoint.BP_RespawnPoint_C")) ; Find Respawn Point
      (set `local.Respawn Points Found` _outactors))
    (:`then_1`
      (if (not (`KismetArrayLibrary.Array_IsEmpty` (`local.Respawn Points Found`)))
        (bind _defaultpawnclass (`self.DefaultPawnClass`)
          (:`then`
            (bind _returnvalue_2 (`|SpawnActorFromClass` _defaultpawnclass (`KismetMathLibrary.MakeTransform` (.location _returnvalue) (`KismetMathLibrary.MakeRotator` 0.0 (.pitch (.rotation _returnvalue)) (.yaw (.rotation _returnvalue)))) "AdjustIfPossibleButAlwaysSpawn" "MultiplyWithRoot" null null :!pinned true)) ; Spawns a new character pawn
            (set `local.SpawnedPawn` _returnvalue_2)
            (`Controller.Possess` (`local.PC`) (`local.SpawnedPawn`) :!pinned true) ; Posess the new character
            (message `/Game/VisualSandbox/Blueprints/Interfaces/BPI_Useful.On Respawn` (`local.PC`)))
          (:`else`))))))

(fn `Set Pause Game`
  (params (Pause :type Boolean))
  (returns (`Return Paused` :type Boolean))
  (return false))

(fn `UserConstructionScript`)