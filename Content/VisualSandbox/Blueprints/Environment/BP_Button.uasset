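; BP_Button is an interactable environment button that triggers other objects when pressed.
; On interaction, it forwards the interaction actor and instigator to every entry in its trigger list, calls its button-pressed event and plays a pressing sound at its location.
; Its health, inventory and item-use functions are empty stubs.
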(event `/Game/VisualSandbox/Blueprints/Interfaces/BPI_Useful.Receive Interaction`
  (params (`Interaction Actor` :type "Actor Object Reference") (`Interaction Instigator` :type "Controller Object Reference"))
  ; On buttom is pressed
  (for _array_element (`self.Trigger Objects`)
    (message `/Game/VisualSandbox/Blueprints/Interfaces/BPI_Useful.Receive Interaction` _array_element `Interaction Actor` `Interaction Instigator`))
  (`self.On Button Pressed` `Interaction Actor` `Interaction Instigator`)
  (`GameplayStatics.PlaySoundAtLocation` (`self.Pressing Sound`) (`self.K2_GetActorLocation`) (struct) 1.0 1.0 0.0 null null null null))

(fn `Get Health System`
  (returns (`Health Conp` :type "/Game/VisualSandbox/Blueprints/Components/AC_HealthComponent Object Reference"))
  (return null))

(fn `Get Inventory System`
  (returns (`Inventory Comp` :type "/Game/VisualSandbox/Blueprints/Components/AC_InventoryComponent Object Reference"))
  (return null))

(fn `Use Item`
  (params (`Item To Use` :type "/Game/VisualSandbox/Blueprints/Pickups/Items/BP_Item Object Reference"))
  (returns (Successful :type Boolean))
  (return false))

(fn `UserConstructionScript`)