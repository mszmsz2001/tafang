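; Explosive barrel prop that detonates when it hits something at high speed after being thrown.
; OnThrowing flags the barrel as thrown and stores the throwing instigator.
; On Hit, a thrown barrel moving above a speed threshold calls Explode with that instigator; any other hit clears both the flag and instigator.
; The explosion logic itself is not defined in these graphs.
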(event `self.ReceiveHit`
  (params (MyComp :type "PrimitiveComponent Object Reference") (Other :type "Actor Object Reference") (OtherComp :type "PrimitiveComponent Object Reference") (bSelfMoved :type Boolean) (HitLocation :type "Vector Structure") (HitNormal :type "Vector Structure") (NormalImpulse :type "Vector Structure") (Hit :type "HitResult Structure (by ref)"))
  ; Explode on impact
  (if (and (`self.Thrown`) (> (`KismetMathLibrary.VSize` (`self.GetVelocity`)) 1500.0))
    (`self.Explode` (`self.Thrown Instigator`))
    (else
      (set `self.Thrown` false)
      (set `self.Thrown Instigator` null))))

(event `/Game/VisualSandbox/Blueprints/Interfaces/BPI_Physics.On Throwing`
  (params (`Throwing Instigator` :type "Controller Object Reference"))
  ; Explode on impact
  (set `self.Thrown Instigator` `Throwing Instigator`)
  (set `self.Thrown` true))

(fn `UserConstructionScript`)