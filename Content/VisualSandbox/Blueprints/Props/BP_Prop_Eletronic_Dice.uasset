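; Electronic dice prop whose dots change emissive color when a pawn hits it.
; The construction script creates a dynamic material instance on the dice mesh.
; On a hit, only the server sets the replicated DotColor from a random color function.
; Its RepNotify writes that color to the material's dot emissive parameter, keeping the look in sync across the network.
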(event `self.Dice Mesh.OnComponentHit`
  (params (HitComponent :type "PrimitiveComponent Object Reference") (OtherActor :type "Actor Object Reference") (OtherComp :type "PrimitiveComponent Object Reference") (NormalImpulse :type "Vector Structure") (Hit :type "HitResult Structure (by ref)"))
  (`/Engine/EditorBlueprintResources/ActorMacros.Switch Has Authority`
    (:`Authority`
      (cast `Pawn` OtherActor)
      (set `self.Dot Color` (`KismetMathLibrary.MakeColor` (`KismetMathLibrary.FMin` (`KismetMathLibrary.RandomFloat`) 1.0) (`KismetMathLibrary.FMin` (`KismetMathLibrary.RandomFloat`) 1.0) (`KismetMathLibrary.FMin` (`KismetMathLibrary.RandomFloat`) 1.0))))))

(fn `OnRep_Dot Color`
  (`MaterialInstanceDynamic.SetVectorParameterValue` (`self.Dice Color`) "Dots Emissive Color" (`self.Dot Color`)))

(fn `UserConstructionScript`
  (bind _returnvalue (`PrimitiveComponent.CreateDynamicMaterialInstance` (`self.Dice Mesh`) 0 "/Game/VisualSandbox/3DAssets/Props/Materials/M_Eletronic_Dice.M_Eletronic_Dice" "None"))
  (set `self.Dice Color` _returnvalue))