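; Custom car vehicle Blueprint that adds configurable neon lighting on top of its parent class.
; The construction script runs the parent's setup, then applies the NeonColor variable to the NeonR and NeonL lights.
; The event graph holds only disabled placeholder events, so the Blueprint adds no runtime logic of its own.
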(fn `UserConstructionScript`
  (`parent.UserConstructionScript`)
  ; Set Neon color
  (for _array_element (`|MakeArray` (`self.Neon R`) (`self.Neon L`))
    (`LightComponent.SetLightColor` _array_element (`self.Neon Color`) true)))