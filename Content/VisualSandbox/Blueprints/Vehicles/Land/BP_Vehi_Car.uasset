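; Drivable Chaos wheeled car pawn with Enhanced Input driving, RPM-driven engine audio, material brake lights, switchable first/third-person cameras and run-over messages to overlapped actors.
; Entering possesses the car, adds its input mapping, attaches the driver and re-registers AI sight.
; Exiting traces exit sockets for capsule clearance, launches the driver with car velocity, then repossesses them after a delay.
; Team index comes from the driver.
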(event `self.ReceiveTick`
  (params (DeltaSeconds :type "Float (single-precision)"))
  ; Set Camera Spring Arm Location
  (`SceneComponent.K2_SetWorldLocation` (`self.SpringArm`) (+ (`self.K2_GetActorLocation`) (0.0 0.0 150.0)) false false) ; fix spring amr
  (`self.Play Engine Sound`))

(event `EnhancedInput|/Game/VisualSandbox/Blueprints/Inputs/Vehicles/IA_Handbrake`
  (params (ActionValue :type Boolean) (ElapsedSeconds :type "Float (double-precision)") (TriggeredSeconds :type "Float (double-precision)") (InputAction :type "InputAction Object Reference" :default "/Game/VisualSandbox/Blueprints/Inputs/Vehicles/IA_Handbrake.IA_Handbrake"))
  ; Braking / Hanbrake
  (:`Started`
    (`self.Handbrake` true))
  (:`Completed`
    (`self.Handbrake` false)))

(event `EnhancedInput|/Game/VisualSandbox/Blueprints/Inputs/Vehicles/IA_Steering`
  (params (ActionValue :type "Float (double-precision)") (ElapsedSeconds :type "Float (double-precision)") (TriggeredSeconds :type "Float (double-precision)") (InputAction :type "InputAction Object Reference" :default "/Game/VisualSandbox/Blueprints/Inputs/Vehicles/IA_Steering.IA_Steering"))
  (bind _vehiclemovementcomponent (`self.VehicleMovementComponent`))
  ; Steering
  (:`Triggered`
    (`ChaosVehicleMovementComponent.SetSteeringInput` _vehiclemovementcomponent ActionValue))
  (:`Completed`
    (`ChaosVehicleMovementComponent.SetSteeringInput` _vehiclemovementcomponent 0.0)))

(event `EnhancedInput|/Game/VisualSandbox/Blueprints/Inputs/Vehicles/IA_Brake`
  (params (ActionValue :type "Float (double-precision)") (ElapsedSeconds :type "Float (double-precision)") (TriggeredSeconds :type "Float (double-precision)") (InputAction :type "InputAction Object Reference" :default "/Game/VisualSandbox/Blueprints/Inputs/Vehicles/IA_Brake.IA_Brake"))
  ; Braking / Hanbrake
  (:`Triggered`
    (`self.Brake` ActionValue))
  (:`Completed`
    (`self.Brake` ActionValue)))

(event `EnhancedInput|/Game/VisualSandbox/Blueprints/Inputs/Vehicles/IA_Accelerate`
  (params (ActionValue :type "Float (double-precision)") (ElapsedSeconds :type "Float (double-precision)") (TriggeredSeconds :type "Float (double-precision)") (InputAction :type "InputAction Object Reference" :default "/Game/VisualSandbox/Blueprints/Inputs/Vehicles/IA_Accelerate.IA_Accelerate"))
  ; Accelerate
  (:`Triggered`
    (`self.Accelerate` 1.0))
  (:`Completed`
    (`self.Accelerate` 0.0)))

(event `self.ReceiveBeginPlay`
  ; Begin Play
  (bind `_aschaos轮式载具运动组件` (cast `ChaosWheeledVehicleMovementComponent` (`self.VehicleMovementComponent`)))
  (set `self.Chaos Wheeled Vehicle Movement Component` `_aschaos轮式载具运动组件`))

(event `/Game/VisualSandbox/Blueprints/Interfaces/BPI_Vehicle.Get Into The Vehicle`
  (params (Character :type "Character Object Reference"))
  ; Get in the car
  (`self.Get In The Car` Character))

(event `self.Mesh.OnComponentBeginOverlap`
  (params (OverlappedComponent :type "PrimitiveComponent Object Reference") (OtherActor :type "Actor Object Reference") (OtherComp :type "PrimitiveComponent Object Reference") (OtherBodyIndex :type Integer) (bFromSweep :type Boolean) (SweepResult :type "HitResult Structure (by ref)"))
  ; Run Over
  (message `/Game/VisualSandbox/Blueprints/Interfaces/BPI_Physics.On Running Over` OtherActor self (`self.GetInstigatorController`)))

(event `Key|One`
  (params (Key :type "Key Structure"))
  ; Switch Camera
  (:`Pressed`
    (`ActorComponent.SetActive` (`self.1P Camera`) false false)
    (`ActorComponent.SetActive` (`self.3P Camera`) false false)
    (`/Engine/EditorBlueprintResources/StandardMacros.FlipFlop`
      (:`A`
        (`ActorComponent.SetActive` (`self.1P Camera`) true false))
      (:`B`
        (`ActorComponent.SetActive` (`self.3P Camera`) true false)))))

(event `EnhancedInput|/Game/VisualSandbox/Blueprints/Inputs/Vehicles/IA_Exit_Vehicle`
  (params (ActionValue :type Boolean) (ElapsedSeconds :type "Float (double-precision)") (TriggeredSeconds :type "Float (double-precision)") (InputAction :type "InputAction Object Reference" :default "/Game/VisualSandbox/Blueprints/Inputs/Vehicles/IA_Exit_Vehicle.IA_Exit_Vehicle"))
  ; Exit the car
  (:`Started`
    (`self.Exit The Car`)
    (`KismetSystemLibrary.Delay` 0.2)
    (`Controller.Possess` (`self.GetController`) (`self.Driver Pawn`)) ; possess back the driver
    (set `self.Driver Pawn` null :!pinned true) ; Clear driver reference
  ))

(fn `Accelerate`
  (params (`Acceleration Force` :type "Float (double-precision)"))
  (locals (`Is Accelerating` :type Boolean))
  (`ChaosVehicleMovementComponent.SetThrottleInput` (`self.VehicleMovementComponent`) (`local.Acceleration Force`)))

(fn `Brake`
  (params (`Braking Force` :type "Float (double-precision)"))
  (locals (`Is Braking` :type Boolean))
  (bind _output_get (set `local.Is Braking` (> `Braking Force` 0.0)))
  (`self.Brake Lights` _output_get)
  (`ChaosVehicleMovementComponent.SetBrakeInput` (`self.VehicleMovementComponent`) (`local.Braking Force`)))

(fn `Brake Lights`
  (params (`Is Braking` :type Boolean))
  (`MaterialInstanceDynamic.SetScalarParameterValue` (`self.Mesh Material`) "BrakeLightPower" (`KismetMathLibrary.SelectFloat` 200.0 4.0 `Is Braking`)))

(fn `Can Enter`
  (params (Driver :type "Character Object Reference"))
  (returns (Successful :type Boolean) (`Fail Reason` :type String))
  (`self.Driver Pawn`
    (:`then`)
    (:`else`
      (return true "Already has a driver"))))

(fn `Can Enter The Vehicle`
  (params (Character :type "Character Object Reference"))
  (returns (Successful :type Boolean) (`Fail Reason` :type String))
  (bind (_successful _fail_reason) (`self.Can Enter` Character))
  (return _successful _fail_reason))

(fn `Exit The Car`
  (`self.Driver Pawn`
    (:`then`
      ; Check exit point
      (if (`KismetArrayLibrary.Array_IsNotEmpty` (`self.Get Exit Points`))
        ; Remove car controls inputs from the player controller
        (message `/Game/VisualSandbox/Blueprints/Interfaces/BPI_Game.Remove IMC Asset` (`self.GetController`) (`self.Car IMC Asset`))
        ; Relocate the driver pawn to out side of the car
        (`self.K2_SetActorLocationAndRotation` :`self` (`self.Driver Pawn`) :`NewLocation` (`|GetArrayItem` (`self.Get Exit Points`)) :`bTeleport` true)
        ; Change diver character state
        (message `/Game/VisualSandbox/Blueprints/Interfaces/BPI_Useful.Set Character State` (`self.Driver Pawn`) "NewEnumerator3")
        ; Match character speed with the car
        (`Character.LaunchCharacter` (`self.Driver Pawn`) (`self.GetVelocity`) false false)))
    (:`else`)))

(fn `Get Exit Points`
  (returns (`Exit Points` :type "Array of Vector Structure"))
  (locals (`Exit Socket Location` :type "Vector Structure" :default (0.0 0.0 0.0)) (`Exit Socket Rotation` :type "Rotator Structure" :default (struct)) (`Exit Points Found` :type "Array of Vector Structure"))
  (bind _exit_socket_location (`local.Exit Socket Location`))
  (bind _capsulecomponent (`Character.CapsuleComponent` (`self.Driver Pawn`)))
  (bind _capsulehalfheight (`CapsuleComponent.CapsuleHalfHeight` _capsulecomponent))
  (for _array_element (`self.Exit Socket Name`)
    (bind (_returnvalue_location _returnvalue_rotation) (`KismetMathLibrary.BreakTransform` (`SceneComponent.GetSocketTransform` (`self.Mesh`) _array_element "RTS_World")))
    (set `local.Exit Socket Location` _returnvalue_location)
    (set `local.Exit Socket Rotation` _returnvalue_rotation)
    (bind (_outhit _returnvalue) (`KismetSystemLibrary.LineTraceSingle` (+ _exit_socket_location (0.0 0.0 100.0)) (- _exit_socket_location (0.0 0.0 100.0)) "TraceTypeQuery1"))
    (bind _returnvalue_2 (+ (`KismetMathLibrary.SelectVector` (`.Location` (`GameplayStatics.BreakHitResult` _outhit)) (`local.Exit Socket Location`) _returnvalue) (`KismetMathLibrary.MakeVector` 0.0 0.0 _capsulehalfheight)))
    (bind _outhit_2 (`KismetSystemLibrary.CapsuleTraceSingle` :`Start` _returnvalue_2 :`End` _returnvalue_2 :`Radius` (`CapsuleComponent.GetScaledCapsuleRadius` _capsulecomponent) :`HalfHeight` (- _capsulehalfheight 20.0) :`TraceChannel` "TraceTypeQuery2" :`bIgnoreSelf` false))
    (if (not (`GameplayStatics.BreakHitResult` _outhit_2))
      (`KismetArrayLibrary.Array_Add` (`local.Exit Points Found`) (`.TraceStart` (`GameplayStatics.BreakHitResult` _outhit_2)))))
  (return (`local.Exit Points Found`)))

(fn `Get In The Car`
  (params (`New Driver` :type "Character Object Reference"))
  (bind _aiperceptionstimulisource (`self.AIPerceptionStimuliSource`))
  (bind _output_get (set `self.Driver Pawn` `New Driver`))
  ; Possess the car
  (`Controller.Possess` (`self.GetController` _output_get) self)
  ; Register car IMC Asset
  (message `/Game/VisualSandbox/Blueprints/Interfaces/BPI_Game.Add IMC Asset` (`self.GetController`) (`self.Car IMC Asset`) 0) ; Add car controls
  ; Update AI Sense for AI perception
  (`AIPerceptionStimuliSourceComponent.UnregisterFromSense` _aiperceptionstimulisource "/Script/AIModule.AISense_Sight")
  (`AIPerceptionStimuliSourceComponent.RegisterForSense` _aiperceptionstimulisource "/Script/AIModule.AISense_Sight")
  ; Change character state to driving
  (message `/Game/VisualSandbox/Blueprints/Interfaces/BPI_Useful.Set Character State` (`self.Driver Pawn`) "NewEnumerator0")
  (`self.K2_AttachToActor` (`self.Driver Pawn`) self "None" "SnapToTarget" "KeepWorld" "KeepWorld" true))

(fn `Get Team Index`
  (returns (ReturnValue :type Integer))
  (bind _driver_pawn (`self.Driver Pawn`)
    (:`then`
      (bind _returnvalue (message `/Game/VisualSandbox/Blueprints/Interfaces/BPI_Bot.Get Team Index` _driver_pawn))
      (return _returnvalue))
    (:`else`
      (return -1))))

(fn `Handbrake`
  (params (Pull :type Boolean))
  (`ChaosVehicleMovementComponent.SetHandbrakeInput` (`self.VehicleMovementComponent`) Pull))

(fn `Has Ammo`
  (returns (Return :type Boolean))
  (return false))

(fn `Is Alive`
  (returns (ReturnValue :type Boolean))
  (return true))

(fn `Play Engine Sound`
  (bind _engine_sound (`self.Engine Sound`))
  (bind _output_get (set `self.Engine RPM` (`ChaosWheeledVehicleMovementComponent.GetEngineRotationSpeed` (`self.Chaos Wheeled Vehicle Movement Component`))))
  (if (< _output_get 600.0)
    (`AudioComponent.SetFloatParameter` _engine_sound "RPM" 600.0)
    (else
      (`AudioComponent.SetFloatParameter` _engine_sound "RPM" (`self.Engine RPM`)))))

(fn `UserConstructionScript`
  (bind _returnvalue (`PrimitiveComponent.CreateDynamicMaterialInstance` (`self.Mesh`) 0 null "None"))
  (set `self.Mesh Material` _returnvalue))