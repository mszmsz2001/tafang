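; BP_Item_Skeletal is a pickup item variant that uses a skeletal mesh with physics when dropped.
; Construction caches the mesh's relative transform and attaches the Sensor and widget component to it.
; Pickup disables physics and collision, then reattaches the skeletal mesh to ItemMesh at the cached transform.
; Dropping restores the item collision profile and re-enables physics simulation, extending the parent's pickup and drop logic.
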(fn `On Dropping`
  (`parent.On Dropping`)
  (`PrimitiveComponent.SetCollisionProfileName` (`self.Item Skeletal Mesh`) (`self.Item Collision Profile Name`) true)
  (`PrimitiveComponent.SetSimulatePhysics` (`self.Item Skeletal Mesh`) true))

(fn `On Picking Up`
  (params (`New Owner` :type "Actor Object Reference"))
  (bind _item_skeletal_mesh (`self.Item Skeletal Mesh`))
  (`parent.On Picking Up` `New Owner`)
  (`PrimitiveComponent.SetSimulatePhysics` _item_skeletal_mesh false) ; stop physics simulation
  (`PrimitiveComponent.SetCollisionEnabled` _item_skeletal_mesh "NoCollision")
  (`SceneComponent.K2_AttachToComponent` (`self.Item Skeletal Mesh`) (`self.Item Mesh`) "None" "SnapToTarget" "SnapToTarget" "KeepWorld" true)
  (`SceneComponent.K2_SetRelativeTransform` (`self.Item Skeletal Mesh`) (`self.Initial Position`) true true))

(fn `UserConstructionScript`
  (`parent.UserConstructionScript`)
  (set `self.Initial Position` (`SceneComponent.GetRelativeTransform` (`self.Item Skeletal Mesh`)))
  (for _array_element (`|MakeArray` (`self.Sensor`) (`self.SC_ActorWidgetComponent`) :!type "SceneComponent Object Reference")
    (`SceneComponent.K2_AttachToComponent` _array_element (`self.Item Skeletal Mesh`) "None" "SnapToTarget" "SnapToTarget" "KeepRelative" true)))