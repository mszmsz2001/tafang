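; Base pickup item that holds a consumable amount and switches between lying in the world and being owned.
; UseItem checks usability and amount, calls the overridable effect, consumes one unit and has the inventory component drop and destroy the item when empty.
; Pickup and drop functions toggle ownership, sensor collision, mesh physics and widget visibility, with unowned items dropped on authority at BeginPlay.
; CanUse, ApplyItemEffect and equip hooks are stubs for child items.
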(event `self.ReceiveBeginPlay`
  ; Begin Play
  (`/Engine/EditorBlueprintResources/ActorMacros.Switch Has Authority`
    (:`Authority`
      (if (not (`self.Has Owner`))
        (`self.On Dropping`)))))

(fn `Add Amount`
  (params (`Amount to Add` :type Integer))
  (set `self.Content Amount` (`KismetMathLibrary.Clamp` (+ (`self.Content Amount`) (`local.Amount to Add`)) 0 (`self.Max Content Amount`))))

(fn `Apply Item Effect`
  (params (User :type "Actor Object Reference")))

(fn `Can Use`
  (params (User :type "Actor Object Reference"))
  (returns (ReturnValue :type Boolean))
  (return false))

(fn `Consume Amount`
  (params (`Amount to Consume` :type Integer))
  (set `self.Content Amount` (`KismetMathLibrary.Max` (- (`self.Content Amount`) (`local.Amount to Consume`)))))

(fn `Get Amount`
  (returns (ReturnValue :type Integer))
  (return (`self.Content Amount`)))

(fn `Get Avaliable Space`
  (returns (ReturnValue :type Integer))
  (return (`KismetMathLibrary.Max` (- (`self.Get Max Amount`) (`self.Get Amount`)))))

(fn `Get Max Amount`
  (returns (ReturnValue :type Integer))
  (return (`self.Max Content Amount`)))

(fn `Has Owner`
  (returns (ReturnValue :type Boolean))
  (`/Engine/EditorBlueprintResources/StandardMacros.IsValid` (`self.GetOwner`)
    (:`Is Valid`
      (return true))
    (:`Is Not Valid`
      (return false))))

(fn `Is Empty`
  (returns (ReturnValue :type Boolean))
  (return (<= (`self.Get Amount`) 0)))

(fn `Is Full`
  (returns (ReturnValue :type Boolean))
  (return (>= (`self.Get Amount`) (`self.Get Max Amount`))))

(fn `On Dropping`
  (`PrimitiveComponent.SetCollisionEnabled` (`self.Sensor`) "QueryOnly")
  (`self.SetOwner` null)
  (`self.K2_DetachFromActor` "KeepWorld" "KeepWorld" "KeepWorld")
  (`self.SetActorHiddenInGame` false)
  (`PrimitiveComponent.SetCollisionProfileName` (`self.Item Mesh`) (`self.Item Collision Profile Name`) true)
  (`PrimitiveComponent.SetSimulatePhysics` (`self.Item Mesh`) true)
  (`SceneComponent.SetVisibility` (`self.SC_ActorWidgetComponent`) true false)
  (set `self.Inventory Comp` null))

(fn `On Equipping`)

(fn `On Picking Up`
  (params (`New Owner` :type "Actor Object Reference"))
  (bind _item_mesh (`self.Item Mesh`))
  (`self.SetOwner` `New Owner`)
  (`PrimitiveComponent.SetCollisionEnabled` (`self.Sensor`) "NoCollision")
  (`PrimitiveComponent.SetSimulatePhysics` _item_mesh false)
  (`PrimitiveComponent.SetCollisionEnabled` _item_mesh "NoCollision")
  (`SceneComponent.SetVisibility` (`self.SC_ActorWidgetComponent`) false false))

(fn `On Unequipping`)

(fn `Set Amount`
  (params (`New Value` :type Integer))
  (returns (`New Amount` :type Integer))
  (bind _output_get (set `self.Content Amount` `New Value`))
  (return _output_get))

(fn `Use Item`
  (params (User :type "Actor Object Reference"))
  (`/Engine/EditorBlueprintResources/StandardMacros.IsValid` User
    (:`Is Valid`
      (if (and (`self.Can Be Used`) (`self.Can Use` (`local.User`)) (not (`self.Is Empty`)))
        (`self.Apply Item Effect` (`local.User`))
        (`self.Consume Amount` 1)
        ;[1 1 1] Drop item when get empty
        (`self.Inventory Comp`
          (:`then`
            (if (`self.Is Empty`)
              (`/Game/VisualSandbox/Blueprints/Components/AC_InventoryComponent.Drop Item` (`self.Inventory Comp`) self true)))
          (:`else`))))))

(fn `UserConstructionScript`)