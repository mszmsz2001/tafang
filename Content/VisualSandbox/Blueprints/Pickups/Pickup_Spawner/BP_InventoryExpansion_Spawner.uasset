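; Pickup spawner that expands a shooter character's inventory by a set number of additional slots.
; Pick Up casts the recipient to BP_ShooterCharacter and resizes its CharacterInventory to the current size plus AdditionalSlots.
; Can Pick Up allows collection only while the inventory is below its maximum size and AdditionalSlots is positive, with an empty fail reason.
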(fn `Can Pick Up`
  (returns (ReturnValue :type Boolean) (`Fail Reason` :type String))
  (bind _asbp_shooter_character (cast `/Game/VisualSandbox/Blueprints/Characters/BP_ShooterCharacter` (`self.Recipient`)))
  (bind _character_inventory (`/Game/VisualSandbox/Blueprints/Characters/BP_ShooterCharacter.Character Inventory` _asbp_shooter_character))
  (return (and (< (`/Game/VisualSandbox/Blueprints/Components/AC_InventoryComponent.Get Inventory Size` _character_inventory) (`/Game/VisualSandbox/Blueprints/Components/AC_InventoryComponent.Inventory Max Size` _character_inventory)) (> (`self.Additional Slots`) 0)) ""))

(fn `Pick Up`
  (bind _asbp_shooter_character (cast `/Game/VisualSandbox/Blueprints/Characters/BP_ShooterCharacter` (`self.Recipient`)))
  (bind _character_inventory (`/Game/VisualSandbox/Blueprints/Characters/BP_ShooterCharacter.Character Inventory` _asbp_shooter_character))
  (`/Game/VisualSandbox/Blueprints/Components/AC_InventoryComponent.Resize Inventory` _character_inventory (+ (`/Game/VisualSandbox/Blueprints/Components/AC_InventoryComponent.Get Inventory Size` _character_inventory) (`self.Additional Slots`))))

(fn `UserConstructionScript`
  (`parent.UserConstructionScript`))