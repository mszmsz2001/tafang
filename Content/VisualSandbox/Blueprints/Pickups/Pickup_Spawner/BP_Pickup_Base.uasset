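; Base pickup actor that hands its effect to an overlapping actor, then hides and optionally respawns after a timer.
; Child classes supply CanPickUp and PickUp, which are stubs here, with CanPickUp failing by default.
; Overlap runs PickUp and its sound on every machine, while only the server toggles PickupActivated and starts the respawn timer.
; The PickupActivated RepNotify drives visibility, collision and the respawn sound.
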(event `Respawning Item`
  ;[0.15 0.15 1 0.5] Respawning process
  (set `self.Pickup Activated` true))

(event `self.Collison.OnComponentBeginOverlap`
  (params (OverlappedComponent :type "PrimitiveComponent Object Reference") (OtherActor :type "Actor Object Reference") (OtherComp :type "PrimitiveComponent Object Reference") (OtherBodyIndex :type Integer) (bFromSweep :type Boolean) (SweepResult :type "HitResult Structure (by ref)"))
  (bind (_returnvalue _fail_reason) (`self.Can Pick Up`))
  ;[1 0.6317 0.15 0.5] On the Pick up begin overlap  (Run on all connected players)
  (set `self.Recipient` OtherActor)
  (if _returnvalue
    (`|ExecutionSequence`
      (:`then_0`
        ;[0.15 0.15 1 0.5] Deactivate and set respawn timer (Run only on the server)
        (`/Engine/EditorBlueprintResources/ActorMacros.Switch Has Authority`
          (:`Authority`
            (set `self.Pickup Activated` false)
            (if (`self.Can Respawn`)
              (`KismetSystemLibrary.K2_SetTimer` null "Respawning Item" (`self.Respawn Time`)) ; set timer for respawn
            ))))
      (:`then_1`
        (`self.Pick Up`) ; apply floating item effect
        (`GameplayStatics.PlaySoundAtLocation` (`self.Pick Up Sound`) (`self.K2_GetActorLocation`) (struct) 1.0 1.0 0.0 null null null null) ; Play picking up sound
      ))
    (else
      (`KismetSystemLibrary.PrintString` _fail_reason true true (struct :`R` 1.0 :`G` 0.004 :`A` 1.0)) ; Debug fail reason
    )))

(fn `Can Pick Up`
  (returns (ReturnValue :type Boolean) (`Fail Reason` :type String))
  (return false ""))

(fn `OnRep_Pickup Activated`
  (if (`self.Pickup Activated`)
    (`GameplayStatics.PlaySoundAtLocation` (`self.Respawning Sound`) (`self.K2_GetActorLocation`) (struct) 1.0 1.0 0.0 null null null null)
    (`self.SetActorHiddenInGame` false)
    (`self.SetActorEnableCollision` true)
    (else
      (`self.SetActorHiddenInGame` true)
      (`self.SetActorEnableCollision` false))))

(fn `Pick Up`)

(fn `UserConstructionScript`)