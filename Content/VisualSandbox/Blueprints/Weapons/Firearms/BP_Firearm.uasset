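; Base firearm item that fires projectiles through its ProjShooter component, with ammo, firing animation, ejection FX, dry-fire sound and shot/empty events.
; A timer derived from RateOfFire gates each shot and re-fires while a fully automatic trigger is held.
; Optional camera or control-rotation traces correct aim within a tolerance of muzzle direction.
; Firing deducts rounds only on authority; dropping resets alignment and unbinds events.
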(event `PlayShootingAnim`
  ; Play Weapon Mesh Shooting Animation
  (`|PlayMontage` (`self.Item Skeletal Mesh`) (`self.Firing Animation`)))

(event `Press Trigger`
  (params (Pressed :type Boolean))
  ; Pull the trigger
  (bind _output_get (set `self.Trigger Pressed` Pressed))
  (if _output_get
    (`self.Fire`)))

(fn `Add Rounds`
  (params (AddAmount :type Integer))
  (`/Engine/EditorBlueprintResources/ActorMacros.Switch Has Authority`
    (:`Authority`
      (set `self.Rounds` (`KismetMathLibrary.Clamp` (+ (`self.Rounds`) (`KismetMathLibrary.Abs_Int` (`local.AddAmount`))) 0 (`self.Max Rounds`))))))

(fn `Calc Shot Correction Direction`
  (params (`Actors To Ignore` :type "Array of Actor Object Reference"))
  (returns (ReturnValue :type "Rotator Structure"))
  (locals (IsBlocking :type Boolean :default false) (TraceStartLocation :type "Vector Structure") (TraceEndLocation :type "Vector Structure") (DesiredRotation :type "Rotator Structure" :default (struct)))
  (bind (_outlocation _outrotation) (`self.GetActorEyesViewPoint` (select `/Game/VisualSandbox/Blueprints/Enumerations/EShotAlignmentMode` (`self.Shot Alignment Mode`) :`NewEnumerator0` (`GameplayStatics.GetPlayerCameraManager` 0) :`NewEnumerator1` (`self.GetOwner`) :!type "Actor Object Reference")))
  (if (> (`self.Shot Alignment Mode`) 0)
    (`|ExecutionSequence`
      (:`then_0`
        (set `local.TraceStartLocation` (+ _outlocation (* (`KismetMathLibrary.GetForwardVector` _outrotation) (`self.Shot Corretion Start Distance`))))
        (set `local.TraceEndLocation` (+ _outlocation (* (`KismetMathLibrary.GetForwardVector` _outrotation) (`self.Shot Corretion End Distance`))))
        (`KismetArrayLibrary.Array_AddUnique` (`local.Actors To Ignore`) (`self.GetOwner`))
        (bind _outhit (`KismetSystemLibrary.LineTraceSingle` (`local.TraceStartLocation`) (`local.TraceEndLocation`) "TraceTypeQuery3" false (`local.Actors To Ignore`)))
        (set `local.IsBlocking` (`GameplayStatics.BreakHitResult` _outhit))
        (set `local.DesiredRotation` (`KismetMathLibrary.FindLookAtRotation` (`SceneComponent.K2_GetComponentLocation` (`self.Proj Shooter`)) (`KismetMathLibrary.SelectVector` (`.Location` (`GameplayStatics.BreakHitResult` _outhit)) (`.TraceEnd` (`GameplayStatics.BreakHitResult` _outhit)) (`local.IsBlocking`)))))
      (:`then_1`
        (return (`KismetMathLibrary.SelectRotator` (`self.Get Muzzle Direction`) (`local.DesiredRotation`) (!= (`local.DesiredRotation`) (`self.Get Muzzle Direction`) :`ErrorTolerance` (`self.Shot Correction Tolerance`))))))
    (else
      (return (`self.Get Muzzle Direction`)))))

(fn `Consume Amount`
  (params (`Amount to Consume` :type Integer))
  (set `self.Rounds` (`KismetMathLibrary.Max` (- (`self.Rounds`) (`local.Amount to Consume`)))))

(fn `Cycling Completed`
  (`KismetSystemLibrary.K2_ClearAndInvalidateTimerHandle` (`self.Cycling Timer`))
  (if (`self.Has Rounds`)
    (if (and (`self.Trigger Pressed`) (`self.Fully Automatic`))
      (`self.Fire`))
    (else
      (`self.OnGetEmpty`))))

(fn `Fire`
  (if (`self.Is Cycling`) :!pinned true
    _
    (elif (or (`self.Has Rounds`) (`self.Infinite Rounds`)) :!pinned true
      (`|ExecutionSequence`
        (:`then_0`
          ;[0.15 0.15 1 0.5] Subtract rounds
          (`/Engine/EditorBlueprintResources/ActorMacros.Switch Has Authority`
            (:`Authority`
              (set `/Game/VisualSandbox/Blueprints/Components/SC_ProjectileShooterComponent.Projectile Damage` (`self.Weapon Damage`) (`self.Proj Shooter`))
              (if (not (`self.Infinite Rounds`))
                (`/Engine/EditorBlueprintResources/StandardMacros.DecrementInt` (`self.Rounds`))))))
        (:`then_1`
          (`/Game/VisualSandbox/Blueprints/Components/SC_ProjectileShooterComponent.Fire Projectile` (`self.Proj Shooter`) (`self.Calc Shot Correction Direction` _) :!pinned true) ; Shoot projectile
          (`NiagaraFunctionLibrary.SpawnSystemAttached` (`self.Ejection FX`) (`self.Item Skeletal Mesh`) (`self.Ejection Port Socket Name`) (0.0 0.0 0.0) (struct) "SnapToTarget" :!pinned true) ; Spawn capsule ejection FX
          (`self.OnShotsFired`)
          (`self.PlayShootingAnim`)
          (bind _returnvalue (`KismetSystemLibrary.K2_SetTimer` null "Cycling Completed" (`self.Get Fire Interval`) :!pinned true)) ; Executes weapon cycling timer
          (set `self.Cycling Timer` _returnvalue)))
      (else
        (`GameplayStatics.PlaySound2D` (`self.Dry Shot`) 1.0 1.0 0.0 null null :!pinned true) ; Plays empty sound
      ))))

(fn `Get Amount`
  (returns (ReturnValue :type Integer))
  (return (`self.Rounds`)))

(fn `Get Avaliable Space`
  (returns (ReturnValue :type Integer))
  (return (`KismetMathLibrary.Max` (- (`self.Max Rounds`) (`self.Rounds`)))))

(fn `Get Fire Interval`
  (returns (ReturnValue :type "Float (double-precision)"))
  (return (/ 60.0 (`self.Rate Of Fire`))))

(fn `Get Max Amount`
  (returns (ReturnValue :type Integer))
  (return (`self.Max Rounds`)))

(fn `Get Muzzle Direction`
  (returns (Rotation :type "Rotator Structure"))
  (return (`SceneComponent.K2_GetComponentRotation` (`self.Proj Shooter`))))

(fn `Has Rounds`
  (returns (ReturnValue :type Boolean))
  (return (> (`self.Rounds`) 0)))

(fn `Is Cycling`
  (returns (ReturnValue :type Boolean))
  (return (`KismetSystemLibrary.K2_IsValidTimerHandle` (`self.Cycling Timer`))))

(fn `Is Empty`
  (returns (ReturnValue :type Boolean))
  (return (not (`self.Has Rounds`))))

(fn `Is Full`
  (returns (ReturnValue :type Boolean))
  (return (>= (`self.Rounds`) (`self.Max Rounds`))))

(fn `On Dropping`
  (`parent.On Dropping`)
  (`self.Press Trigger` false)
  (set `self.Shot Alignment Mode` "NewEnumerator3")
  (clear `self.OnGetEmpty`)
  (clear `self.OnShotsFired`))

(fn `On Unequipping`
  (`parent.On Unequipping`)
  (`self.Press Trigger` false))

(fn `Set Amount`
  (params (`New Value` :type Integer))
  (returns (`New Amount` :type Integer))
  (bind _output_get (set `self.Rounds` (`KismetMathLibrary.Clamp` `New Value` 0 (`self.Get Max Amount`))))
  (return _output_get))

(fn `UserConstructionScript`
  (`parent.UserConstructionScript`))