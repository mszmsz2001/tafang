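; Physics gun weapon that grabs, carries, drops and throws physics-simulated objects.
; The trigger line-traces along corrected aim and attaches simulating hits to a Physics Handle, which follows the Arrow component each Tick.
; With an object held, single-click drops it, while double-click throws it by impulse and notifies the actor.
; Held objects ignore Pawn collision until release restores their profile, and auto-drop on physics loss, unequip or weapon drop.
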(event `self.Press Trigger`
  (params (Pressed :type Boolean))
  ; On pressing the trigger
  (bind _output_get (set `self.Trigger Pressed` Pressed))
  (if _output_get
    (`/Engine/EditorBlueprintResources/StandardMacros.IsValid` (`self.Get Grabbed Object`)
      (:`Is Valid`
        ; Throw or Drop grabbed object
        ; Double click to Thow and Single click to Drop
        (`/Game/VisualSandbox/Blueprints/Utility/BP_UsefulMacros.Double Click` 0.25
          (:`Double`
            (`self.Drop Object` true))
          (:`Single`
            (`self.Drop Object` false))))
      (:`Is Not Valid`
        (`self.Raycast For Object` :!pinned true) ; Raycast to grab objects
      ))))

(event `self.ReceiveTick`
  (params (DeltaSeconds :type "Float (single-precision)"))
  ; Update grabbed object position
  (`self.Update Grabbed Object Location`))

(fn `Drop Object`
  (params (Throw :type Boolean))
  (`|ExecutionSequence`
    (:`then_0`
      (`/Engine/EditorBlueprintResources/StandardMacros.IsValid` (`self.Get Grabbed Object`)
        (:`Is Valid`
          (`|ExecutionSequence`
            (:`then_0`
              ; Throw
              (if (`local.Throw`)
                (`PrimitiveComponent.AddImpulse` (`self.Get Grabbed Object`) (* (`KismetMathLibrary.GetForwardVector` (`self.Calc Shot Correction Direction` (`|MakeArray` (`self.Grabbed Actor`)))) (`self.Throw Force`)) "None" true :!pinned true) ; Apply Throwing force
                (`self.Play Grabber Sound` (`self.Throwing Sound`))
                (bind _grabbed_actor (`self.Grabbed Actor`)
                  (:`then`
                    (message `/Game/ProjectTD/Blueprints/Interfaces/BPI_Physics.On Throwing` _grabbed_actor (`self.GetInstigatorController`)))
                  (:`else`))))
            (:`then_1`
              ; Reset grabbed object collision and clear Grabbed actor reference
              (`PrimitiveComponent.SetCollisionProfileName` (`self.Get Grabbed Object`) (`self.Object Collision Profile`) true)
              (`PhysicsHandleComponent.ReleaseComponent` (`self.PhysicsHandle`))
              (set `self.Grabbed Actor` null))))))
    (:`then_1`
      ; Stop grabbing sound
      (bind _grabber_sound_comp (`self.Grabber Sound Comp`)
        (:`then`
          (`AudioComponent.Stop` _grabber_sound_comp))
        (:`else`)))))

(fn `Get Grabbed Object`
  (returns (ReturnValue :type "PrimitiveComponent Object Reference"))
  (return (`PhysicsHandleComponent.GetGrabbedComponent` (`self.PhysicsHandle`))))

(fn `On Dropping`
  (`parent.On Dropping`)
  (`self.Drop Object` false))

(fn `On Unequipping`
  (`parent.On Unequipping`)
  (`self.Drop Object` false))

(fn `Play Grabber Sound`
  (params (Sound :type "SoundCue Object Reference"))
  (`GameplayStatics.PlaySoundAtLocation` Sound (`self.K2_GetActorLocation`) (struct) 1.0 1.0 0.0 null null null null))

(fn `Raycast For Object`
  (locals (`Component Found` :type "PrimitiveComponent Object Reference") (`Grabbed Location` :type "Vector Structure" :default (0.0 0.0 0.0)) (`Grabbed Bone` :type Name :default "None") (TraceStartLocation :type "Vector Structure" :default (0.0 0.0 0.0)))
  (bind _component_found (`local.Component Found`))
  (bind _grabbed_bone (`local.Grabbed Bone`))
  (`self.Play Grabber Sound` (`self.Raycasting Sound`)) ; Play raycasting sound
  ; Line trace to detect physics simulated objects
  (bind _output_get (set `local.TraceStartLocation` (`SceneComponent.K2_GetComponentLocation` (`self.Proj Shooter`))))
  (bind _outhit (`KismetSystemLibrary.LineTraceSingle` _output_get (+ _output_get (* (`KismetMathLibrary.GetForwardVector` (`self.Calc Shot Correction Direction` _)) (`self.Raycast Distance`))) (`self.Raycast Trace Channel`) false (`|MakeArray` (`self.GetOwner`))))
  (if (`GameplayStatics.BreakHitResult` _outhit)
    (set `local.Grabbed Location` (`.Location` (`GameplayStatics.BreakHitResult` _outhit)))
    (set `self.Grabbed Actor` (`.HitActor` (`GameplayStatics.BreakHitResult` _outhit)))
    (set `local.Component Found` (`.HitComponent` (`GameplayStatics.BreakHitResult` _outhit)))
    (set `local.Grabbed Bone` (`.HitBoneName` (`GameplayStatics.BreakHitResult` _outhit)))
    (if (`SceneComponent.IsSimulatingPhysics` (`local.Component Found`) (`local.Grabbed Bone`))
      ; Save grabbed collision profile
      (set `self.Object Collision Profile` (`PrimitiveComponent.GetCollisionProfileName` (`local.Component Found`)))
      ; Assign grabbed object to the Physics Handle component
      (`PhysicsHandleComponent.GrabComponentAtLocationWithRotation` (`self.PhysicsHandle`) (`local.Component Found`) (`local.Grabbed Bone`) (`local.Grabbed Location`) (`SceneComponent.K2_GetComponentRotation` (`self.Arrow`)))
      ; Neutralize object movements
      (`PrimitiveComponent.SetPhysicsAngularVelocityInDegrees` _component_found (0.0 0.0 0.0) false _grabbed_bone)
      (`PrimitiveComponent.SetPhysicsLinearVelocity` _component_found (0.0 0.0 0.0) false _grabbed_bone)
      ; Ignore pawn collision to prevent collision conflict between player and grabbed object
      (`PrimitiveComponent.SetCollisionResponseToChannel` (`local.Component Found`) "ECC_Pawn" "ECR_Ignore")
      ; Play grabbing sound
      (bind _grabber_sound_comp (`self.Grabber Sound Comp`)
        (:`then`
          (`AudioComponent.Play` _grabber_sound_comp 0.0))
        (:`else`
          (bind _returnvalue (`GameplayStatics.SpawnSoundAttached` (`self.Grabbing Sound`) (`self.Item Skeletal Mesh`) "None" (0.0 0.0 0.0) (struct) "KeepRelativeOffset" false 1.0 1.0 0.0 null null))
          (set `self.Grabber Sound Comp` _returnvalue))))))

(fn `Update Grabbed Object Location`
  (bind _arrow (`self.Arrow`))
  (`/Engine/EditorBlueprintResources/StandardMacros.IsValid` (`self.Get Grabbed Object`)
    (:`Is Valid`
      ; Drop the object if no longer simulationg physics
      (if (`SceneComponent.IsSimulatingPhysics` (`self.Get Grabbed Object`) "None")
        ; Update object location
        (`PhysicsHandleComponent.SetTargetLocationAndRotation` (`self.PhysicsHandle`) (`SceneComponent.K2_GetComponentLocation` _arrow) (`SceneComponent.K2_GetComponentRotation` _arrow))
        (else
          (`self.Drop Object` false))))
    (:`Is Not Valid`
      (`self.Drop Object` false))))

(fn `UserConstructionScript`
  (`parent.UserConstructionScript`))