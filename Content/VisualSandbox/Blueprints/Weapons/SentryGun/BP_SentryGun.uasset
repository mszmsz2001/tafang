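; BP_SentryGun is an AI-controlled, team-indexed sentry turret that shoots projectiles and explodes when destroyed.
; Shoot applies a fire-rate cooldown and calls Fire, which spends ammo on authority, launches a projectile through ProjShooterComp, ejects casings and raises shot or empty callbacks.
; UpdateGunRotation interpolates turret rotation toward a target in actor-local space.
; MachineCondition death triggers Explode, stopping AI on authority, spawning the blast and hiding the actor.
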(event `Shoot`
  (`/Game/VisualSandbox/Blueprints/Utility/BP_UsefulMacros.Cool Down` (`self.Get Fire Interval`)) ; Shooting interval
  (`self.Fire`))

(event `self.Machine Condition.On Dying`
  (params (Instigator :type "Controller Object Reference") (Causer :type "Actor Object Reference"))
  (`self.Explode` :!pinned true) ; Explodes On Dying
)

(fn `Add Rounds`
  (params (AddAmount :type Integer))
  (set `self.Rounds` (`KismetMathLibrary.Clamp` (+ (`self.Rounds`) (`local.AddAmount`)) 0 (`self.Max Rounds`))))

(fn `Explode`
  (`|ExecutionSequence`
    (:`then_0`
      (`/Engine/EditorBlueprintResources/ActorMacros.Switch Has Authority`
        (:`Authority`
          (`self.Stop AI`)
          (`self.SetLifeSpan` 1.0))))
    (:`then_1`
      (`/Game/VisualSandbox/Blueprints/Utility/BP_UsefulFunctions.Spawn Explosion` :`Explosion Origin` (`self.K2_GetActorLocation`) :`Explosion Type` (`self.Explosion Type`) :`Explosion Owner` self :`Explosion Instigator` (`self.GetController`))
      (`self.SetActorHiddenInGame` true)
      (`self.SetActorEnableCollision` false))))

(fn `Fire`
  (bind _return (`self.Has Ammo`))
  (if _return
    (`|ExecutionSequence`
      (:`then_0`
        (`/Engine/EditorBlueprintResources/ActorMacros.Switch Has Authority`
          (:`Authority`
            (if (not (`self.Infinite Rounds`))
              (`/Engine/EditorBlueprintResources/StandardMacros.DecrementInt` (`self.Rounds`)) ; subtracts rounds
            ))))
      (:`then_1`
        (set `/Game/VisualSandbox/Blueprints/Components/SC_ProjectileShooterComponent.Projectile Damage` (`self.Damage`) (`self.Proj Shooter Comp`))
        (`/Game/VisualSandbox/Blueprints/Components/SC_ProjectileShooterComponent.Fire Projectile` :`self` (`self.Proj Shooter Comp`))
        (`NiagaraFunctionLibrary.SpawnSystemAttached` (`self.Capsule Ejection FX`) (`self.Sentry Gun Mesh`) (`self.Ejection Port Socket Name`) (0.0 0.0 0.0) (struct) "SnapToTarget" :!pinned true) ; Spawn capsule ejection effect
        (`self.On Shot Fired`)))
    (else
      (`self.On Get Empty`))))

(fn `Get Fire Interval`
  (returns (ReturnValue :type "Float (double-precision)"))
  (return (/ 60.0 (`self.Fire Rate`))))

(fn `Get Team Index`
  (returns (ReturnValue :type Integer))
  (return (`self.Team Index`)))

(fn `Has Ammo`
  (returns (Return :type Boolean))
  (return (or (> (`self.Rounds`) 0) (`self.Infinite Rounds`))))

(fn `Is Alive`
  (returns (ReturnValue :type Boolean))
  (return (`/Game/VisualSandbox/Blueprints/Components/AC_HealthComponent.Is Alive` (`self.Machine Condition`))))

(fn `Is Full Loaded`
  (returns (ReturnValue :type Boolean))
  (return (>= (`self.Rounds`) (`self.Max Rounds`))))

(fn `Stop AI`
  (bind _braincomponent (`AIController.BrainComponent` (`AIBlueprintHelperLibrary.GetAIController` self))
    (:`then`
      (`BrainComponent.StopLogic` _braincomponent "Is Destroyed"))
    (:`else`)))

(fn `Update Gun Rotation`
  (params (TargetLocation :type "Vector Structure"))
  (locals (`Gun Bone Location` :type "Vector Structure") (`Sentry Gun Transform` :type "Transform Structure") (`Direction World` :type "Vector Structure" :default (0.0 0.0 0.0)) (`Local Direction` :type "Vector Structure" :default (0.0 0.0 0.0)) (`New Turret Rotation` :type "Rotator Structure" :default (struct)))
  (`|ExecutionSequence`
    (:`then_0`
      ; Calcturret rotation
      (set `local.Gun Bone Location` (`SceneComponent.GetSocketLocation` (`self.Sentry Gun Mesh`) "gun"))
      (set `local.Sentry Gun Transform` (`self.GetTransform`))
      (set `local.Direction World` (`KismetMathLibrary.Normal` (- (`local.TargetLocation`) (`local.Gun Bone Location`))))
      (bind _output_get (set `local.Local Direction` (`KismetMathLibrary.InverseTransformDirection` (`local.Sentry Gun Transform`) (`local.Direction World`))))
      (set `local.New Turret Rotation` (`KismetMathLibrary.MakeRotFromX` _output_get)))
    (:`then_1`
      ; Apply turret rotation
      (set `self.Turret Rotation` (`KismetMathLibrary.RInterpTo` (`self.Turret Rotation`) (`local.New Turret Rotation`) (`GameplayStatics.GetWorldDeltaSeconds`) (`self.Turret Rotation Speed`))))))

(fn `UserConstructionScript`
  (`parent.UserConstructionScript`))