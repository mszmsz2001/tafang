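; Rocket projectile Blueprint that explodes when it hits something.
; Its On Impact function spawns an explosion at the rocket's location using its explosion type and radial force, credits the instigator's controller, then destroys the actor.
; The event graph holds only disabled default events, and the construction script just calls its parent.
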(fn `On Impact`
  (params (`Impact Result` :type "HitResult Structure"))
  (`/Game/VisualSandbox/Blueprints/Utility/BP_UsefulFunctions.Spawn Explosion` :`Explosion Origin` (`self.K2_GetActorLocation`) :`Explosion Type` (`self.Explosion Type`) :`Explosion Owner` self :`Explosion Instigator` (`self.GetInstigatorController`) :`Explosion Force` (`self.RadialForce`))
  (`self.K2_DestroyActor`))

(fn `UserConstructionScript`
  (`parent.UserConstructionScript`))