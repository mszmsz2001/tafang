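; BP_MasterCharacter is a base character with movement, health, fall damage and death handling, plus simple default queries for team, ammo, items and inventory.
; Move input follows aim yaw, and landing speed maps to damage as a fraction of max health.
; CharacterHealth's OnDying triggers server-only AI stop, sight unregistration and decompose lifespan, then ragdolls the mesh, disables input and reports the death to the controller.
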(event `self.OnLanded`
  (params (Hit :type "HitResult Structure (by ref)"))
  ; Apply Fall Damage
  (`self.Apply Fall Damage` Hit))

(event `self.Character Health.On Dying`
  (params (Instigator :type "Controller Object Reference") (Causer :type "Actor Object Reference"))
  ; Dying (Run on all connected clients)
  (`self.Dying` Instigator Causer))

(event `EnhancedInput|/Game/VisualSandbox/Blueprints/Inputs/Character/IA_Move`
  (params (ActionValue :type "Vector2D Structure") (ElapsedSeconds :type "Float (double-precision)") (TriggeredSeconds :type "Float (double-precision)") (InputAction :type "InputAction Object Reference" :default "/Game/VisualSandbox/Blueprints/Inputs/Character/IA_Move.IA_Move"))
  ; WASD Movement
  (:`Triggered`
    (`self.WASD Movement` ActionValue)))

(fn `Apply Fall Damage`
  (params (`Impact Info` :type "HitResult Structure"))
  (locals (`Relative Velocity` :type "Vector Structure") (NewLocalVar :type "PrimitiveComponent Object Reference") (`Mass A` :type "Float (double-precision)") (`Mass B` :type "Float (double-precision)") (`Impact Normal` :type "Vector Structure" :default (0.0 0.0 0.0)) (`Relative Speed` :type "Float (double-precision)" :default 0.0) (`Effective Mass` :type "Float (double-precision)") (`Impact Force` :type "Float (double-precision)"))
  (bind (_returnvalue_x _returnvalue_y _returnvalue_z) (`KismetMathLibrary.BreakVector` (`self.GetVelocity`)))
  (`GameplayStatics.ApplyDamage` self (`KismetMathLibrary.Lerp` 0.0 (`/Game/VisualSandbox/Blueprints/Components/AC_HealthComponent.Max Health` (`self.Character Health`)) (`KismetMathLibrary.FClamp` (`KismetMathLibrary.NormalizeToRange` (`KismetMathLibrary.Abs` _returnvalue_z) (`self.Fall Damage Min Speed`) (`self.Fall Damage Fatal Speed`)))) null self))

(fn `Attach To Character`
  (params (Actor :type "Actor Object Reference") (SocketName :type Name))
  (`self.K2_AttachToComponent` Actor (`self.Mesh`) (`local.SocketName`) "SnapToTarget" "SnapToTarget" "KeepRelative" true))

(fn `Can Move`
  (returns (ReturnValue :type Boolean))
  (return true))

(fn `Dying`
  (params (Instigator :type "Controller Object Reference") (Causer :type "Actor Object Reference"))
  (`|ExecutionSequence`
    (:`then_0`
      ;[0.15 0.15 1 0.5] Run only on the server
      (`/Engine/EditorBlueprintResources/ActorMacros.Switch Has Authority`
        (:`Authority`
          (`self.Stop AI`)
          (`self.SetLifeSpan` (`self.Decomposing Time`))
          (`AIPerceptionStimuliSourceComponent.UnregisterFromSense` (`self.AIPerceptionStimuliSource`) "/Script/AIModule.AISense_Sight")
          (set `self.Is Dead` true)
          (set `self.bCanBeDamaged` false))))
    (:`then_1`
      (`self.Start Ragdoll`)
      (`self.DisableInput` null)
      (message `/Game/VisualSandbox/Blueprints/Interfaces/BPI_Useful.Report Pawn Death` (`self.GetController`) (`local.Instigator`) (`local.Causer`))
      (clear `self.OnTakeAnyDamage`))))

(fn `Get Health System`
  (returns (`Health Conp` :type "/Game/VisualSandbox/Blueprints/Components/AC_HealthComponent Object Reference"))
  (return (`self.Character Health`)))

(fn `Get Inventory System`
  (returns (`Inventory Comp` :type "/Game/VisualSandbox/Blueprints/Components/AC_InventoryComponent Object Reference"))
  (return null))

(fn `Get Team Index`
  (returns (ReturnValue :type Integer))
  (return (`self.TeamIndex`)))

(fn `Has Ammo`
  (returns (Return :type Boolean))
  (return false))

(fn `Is Alive`
  (returns (ReturnValue :type Boolean))
  (return (`/Game/VisualSandbox/Blueprints/Components/AC_HealthComponent.Is Alive` (`self.Character Health`))))

(fn `Is Bussy`
  (returns (ReturnValue :type Boolean))
  (return false))

(fn `Save Default Properties`
  (bind _charactermovement (`self.CharacterMovement`))
  (set `self.Default Move Speed` (`CharacterMovementComponent.MaxWalkSpeed` _charactermovement))
  (set `self.Default Move Speed Crouched` (`CharacterMovementComponent.MaxWalkSpeedCrouched` _charactermovement)))

(fn `Set Character Visibility`
  (params (Visible :type Boolean))
  (bind _output_get (set `self.Is Character Visible` Visible))
  (`self.SetActorHiddenInGame` (not _output_get)))

(fn `Start Ragdoll`
  (bind _mesh (`self.Mesh`))
  (if (not (`self.Is Ragdoll`))
    ; Change Mesh collision type and start physics simulation
    (`PrimitiveComponent.SetCollisionProfileName` _mesh "Ragdoll" true)
    (`PrimitiveComponent.SetSimulatePhysics` _mesh true)
    (`PrimitiveComponent.SetCollisionEnabled` (`self.CapsuleComponent`) "NoCollision")
    (`CharacterMovementComponent.SetMovementMode` (`self.CharacterMovement`) "MOVE_None" 0)
    (set `self.Is Ragdoll` true)))

(fn `Stop AI`
  (locals (AI :type "AIController Object Reference"))
  (bind _output_get (set `local.AI` (`AIBlueprintHelperLibrary.GetAIController` self)))
  (`/Engine/EditorBlueprintResources/StandardMacros.IsValid` _output_get
    (:`Is Valid`
      (bind _braincomponent (`AIController.BrainComponent` (`local.AI`))
        (:`then`
          (`BrainComponent.StopLogic` _braincomponent "Dead"))
        (:`else`)))))

(fn `Use Item`
  (params (`Item To Use` :type "/Game/VisualSandbox/Blueprints/Pickups/Items/BP_Item Object Reference"))
  (returns (Successful :type Boolean))
  (return false))

(fn `UserConstructionScript`
  (`self.Save Default Properties`))

(fn `WASD Movement`
  (params (InputValue :type "Vector2D Structure"))
  (bind _returnvalue (`self.GetBaseAimRotation`))
  (bind (_inputvalue_x _inputvalue_y) (`KismetMathLibrary.BreakVector2D` (`local.InputValue`)))
  (if (`self.Can Move`)
    (`|ExecutionSequence`
      (:`then_0`
        (`self.AddMovementInput` (`KismetMathLibrary.GetForwardVector` (`KismetMathLibrary.MakeRotator` 0.0 0.0 (.yaw _returnvalue))) _inputvalue_x))
      (:`then_1`
        (`self.AddMovementInput` (`KismetMathLibrary.GetRightVector` _returnvalue) _inputvalue_y)))))