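; Inventory component that stores items in a fixed-size slot array and creates, opens and closes the inventory widget.
; Adding looks up DT_Item, topping up partial stacks before empty slots; the non-stackable branch writes to every empty slot without breaking.
; Material checks total matching slots, and consumption drains them from the last slot backwards.
; Swapping merges matching stacks up to their limit, and most mutations fire OnInventoryUpdated.
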(event `self.ReceiveBeginPlay`
  (`self.初始化`))

(fn `交换物品`
  (params (FromIndex :type Integer) (ToIndex :type Integer))
  (locals (TotalQuantity :type Integer))
  (bind _slots (`self.Slots`))
  (bind _slots_2 (`self.Slots`))
  (bind _slots_3 (`self.Slots`))
  (bind _fromindex (`local.FromIndex`))
  (bind _toindex (`local.ToIndex`))
  (bind (_output_itemid _output_quantity _output_currentdurability) (break `/Game/ProjectTD_Old/DataStructure/F_InventorySlot` (`|GetArrayItem` _slots ToIndex)))
  (bind (_output_itemid_2 _output_quantity_2) (break `/Game/ProjectTD_Old/DataStructure/F_InventorySlot` (`|GetArrayItem` _slots FromIndex)))
  ; 需要考虑武器、食物药品等物品的交换，这是个简单的写法
  (bind _output_get (set `local.TotalQuantity` (+ _output_quantity_2 _output_quantity)))
  (if (!= _output_itemid_2 _output_itemid)
    (`KismetArrayLibrary.Array_Swap` (`self.Slots`) (`local.FromIndex`) (`local.ToIndex`))
    (else
      (bind _returnvalue (`|GetDataTableRow` "/Game/ProjectTD_Old/DataStructure/DT_Item.DT_Item" _output_itemid)
        (:`then`
          (bind (_displayname _description _icon _itemtype _bisstackable _maxstacksize) (break `/Game/ProjectTD_Old/DataStructure/F_ItemData` _returnvalue))
          (if (<= _output_get _maxstacksize)
            (`KismetArrayLibrary.Array_Set` _slots_3 _toindex (make `/Game/ProjectTD_Old/DataStructure/F_InventorySlot` _output_itemid _output_get _output_currentdurability)) ; 合并
            (`KismetArrayLibrary.Array_Set` _slots_3 _fromindex) ; 清零
            (else
              (`KismetArrayLibrary.Array_Set` _slots_2 _toindex (make `/Game/ProjectTD_Old/DataStructure/F_InventorySlot` _output_itemid _maxstacksize _output_currentdurability)) ; 到上限
              (`KismetArrayLibrary.Array_Set` _slots_2 _fromindex (make `/Game/ProjectTD_Old/DataStructure/F_InventorySlot` _output_itemid (- (`local.TotalQuantity`) _maxstacksize) _output_currentdurability)) ; 补余
            ))))))
  (`self.OnInventoryUpdated`)
  (return))

(fn `关闭背包`
  (`Widget.RemoveFromParent` (`self.InventoryWidget`)))

(fn `初始化`
  (`KismetArrayLibrary.Array_Resize` (`self.Slots`) (`self.MaxSlots`))
  (bind _returnvalue (`|CreateWidget` "/Game/UI/WBP_Inventory.WBP_Inventory_C" (`GameplayStatics.GetPlayerController` 0) self))
  (set `self.InventoryWidget` _returnvalue))

(fn `判断材料是否足够消耗`
  (params (InItemArray :type "Array of /Game/ProjectTD_Old/DataStructure/F_CostItem Structure"))
  (returns (bCanRemove :type Boolean) (OutItemArray :type "Array of /Game/ProjectTD_Old/DataStructure/F_CostItem Structure"))
  (locals (CurrentItemAmount :type Integer :default 0) (AmountToRemove :type Integer) (LastSlotItemNumber :type Integer) (bEnoughRemove :type Boolean))
  (bind _benoughremove (`local.bEnoughRemove`))
  (set `local.bEnoughRemove` false)
  (for _array_element InItemArray
    (bind (_itemrowhandle _quantity) (break `/Game/ProjectTD_Old/DataStructure/F_CostItem` _array_element))
    (set `local.AmountToRemove` _quantity)
    (set `local.CurrentItemAmount` 0)
    (bind (_arrayindex _arrayelement) (`/Game/ProjectTD_Old/Blueprints/BlueprintLibrary/BML_MacroForObject.ReverseForEachLoopWithBreak` (`self.Slots`) :!label _label)
      (:`LoopBody`
        (bind (_itemid _quantity_2) (break `/Game/ProjectTD_Old/DataStructure/F_InventorySlot` _arrayelement))
        (if (== (`.RowName` (break `DataTableRowHandle` _itemrowhandle)) _itemid)
          (set `local.CurrentItemAmount` (+ _quantity_2 (`local.CurrentItemAmount`)))
          (if (>= (`local.CurrentItemAmount`) (`local.AmountToRemove`))
            (set `local.bEnoughRemove` true)
            (goto _label :!via `Break`))))
      (:`Completed`
        (if (not _benoughremove)
          (return _benoughremove)))))
  (return (`local.bEnoughRemove`) InItemArray) ; 正常结束循环
)

(fn `刷新背包物品(UI)`
  (`self.OnInventoryUpdated`)
  (return))

(fn `打开背包`
  (bind _inventorywidget (`self.InventoryWidget`))
  (`/Game/UI/WBP_Inventory.刷新背包UI` _inventorywidget)
  (`UserWidget.AddToViewport` _inventorywidget 0))

(fn `替换某格物品`
  (params (ReplaceItemIndex :type Integer) (ReplaceItem :type "/Game/ProjectTD_Old/DataStructure/F_InventorySlot Structure"))
  (`KismetArrayLibrary.Array_Set` (`self.Slots`) ReplaceItemIndex ReplaceItem)
  (return))

(fn `查询物品数量`
  (params (InItemID :type Name))
  (returns (OutItemAmount :type Integer))
  (locals (CurrentItemAmount :type Integer))
  (set `local.CurrentItemAmount` 0)
  (for _array_element (`self.Slots`)
    (bind (_itemid _quantity) (break `/Game/ProjectTD_Old/DataStructure/F_InventorySlot` _array_element))
    (if (== InItemID _itemid)
      (set `local.CurrentItemAmount` (+ _quantity (`local.CurrentItemAmount`)))))
  (return (`local.CurrentItemAmount`)))

(fn `添加物品`
  (params (InItemID :type Name) (InQuantity :type Integer) (InDurability :type "Float (double-precision)"))
  (returns (OutQuantity :type Integer))
  (locals (AmountToAdd :type Integer) (SpaceAvailable :type Integer) (CurrentMaxStack :type Integer))
  (bind _returnvalue (- (`local.AmountToAdd`) (`local.SpaceAvailable`)))
  (bind _returnvalue_2 (- (`local.AmountToAdd`) (`local.SpaceAvailable`)))
  (set `local.AmountToAdd` InQuantity)
  (bind _returnvalue_3 (`|GetDataTableRow` "/Game/ProjectTD_Old/DataStructure/DT_Item.DT_Item" InItemID)
    (:`then`
      (bind (_displayname _description _icon _itemtype _bisstackable _maxstacksize) (break `/Game/ProjectTD_Old/DataStructure/F_ItemData` _returnvalue_3))
      (set `local.CurrentMaxStack` _maxstacksize)
      (if _bisstackable
        ; 可堆叠物品的添加（多为可消耗材料）
        (for (_array_element _array_index) (`self.Slots`)
          (bind (_itemid _quantity) (break `/Game/ProjectTD_Old/DataStructure/F_InventorySlot` _array_element))
          (if (and (== InItemID _itemid) (> _maxstacksize _quantity))
            (bind _output_get (set `local.SpaceAvailable` (- _maxstacksize _quantity)))
            (`KismetArrayLibrary.Array_Set` (`self.Slots`) _array_index (make `/Game/ProjectTD_Old/DataStructure/F_InventorySlot` (`local.InItemID`) (+ (`KismetMathLibrary.Min` _output_get (`local.AmountToAdd`)) _quantity) (`local.InDurability`)))
            (if (<= _returnvalue_2 0)
              (set `local.AmountToAdd` 0)
              (break)
              (else
                (set `local.AmountToAdd` _returnvalue_2)))))
        (if (not (== (`local.AmountToAdd`) 0))
          (for (_array_element_2 _array_index_2) (`self.Slots`)
            (bind (_itemid_2 _quantity_2) (break `/Game/ProjectTD_Old/DataStructure/F_InventorySlot` _array_element_2))
            (if (== _itemid_2 "None")
              (bind _output_get_2 (set `local.SpaceAvailable` (`local.CurrentMaxStack`)))
              (`KismetArrayLibrary.Array_Set` (`self.Slots`) _array_index_2 (make `/Game/ProjectTD_Old/DataStructure/F_InventorySlot` (`local.InItemID`) (+ (`KismetMathLibrary.Min` _output_get_2 (`local.AmountToAdd`)) _quantity_2) (`local.InDurability`)))
              (if (<= _returnvalue 0)
                (set `local.AmountToAdd` 0)
                (break)
                (else
                  (set `local.AmountToAdd` _returnvalue))))))
        (`self.OnInventoryUpdated`)
        (return 0)
        (else
          ; 不可堆叠物品的添加（一般为枪械、装备等）
          (for (_array_element_3 _array_index_3) (`self.Slots`)
            (if (== (`.ItemID_2_7C14D0294170F80B475BA5B300848896` (break `/Game/ProjectTD_Old/DataStructure/F_InventorySlot` _array_element_3)) "None")
              (`KismetArrayLibrary.Array_Set` (`self.Slots`) _array_index_3 (make `/Game/ProjectTD_Old/DataStructure/F_InventorySlot` InItemID (`local.InQuantity`) (`local.InDurability`))))))))))

(fn `移除某格物品`
  (params (RemoveItemIndex :type Integer))
  (`KismetArrayLibrary.Array_Remove` (`self.Slots`) RemoveItemIndex)
  (return))

(fn `移除物品（消耗材料）`
  (params (bCanRemove :type Boolean) (InCostItemArray :type "Array of /Game/ProjectTD_Old/DataStructure/F_CostItem Structure") (CraftAmount :type Integer :default 1))
  (returns (OutQuantity :type Integer))
  (locals (AmountToRemove :type Integer) (CurrentItemAmount :type Integer) (LastSlotItemNumber :type Integer) (RemoveItemIndexInSlots :type "Array of Integer") (EmptySlot :type "/Game/ProjectTD_Old/DataStructure/F_InventorySlot Structure") (CurrentItemID :type Name))
  (bind _lastslotitemnumber (`local.LastSlotItemNumber`))
  (bind _slots (`self.Slots`))
  (bind _removeitemindexinslots (`local.RemoveItemIndexInSlots`))
  (bind _returnvalue (- (`local.CurrentItemAmount`) (`local.AmountToRemove`)))
  (if bCanRemove
    (for _array_element InCostItemArray
      (bind (_itemrowhandle _quantity) (break `/Game/ProjectTD_Old/DataStructure/F_CostItem` _array_element))
      (set `local.CurrentItemID` (`.RowName` (break `DataTableRowHandle` _itemrowhandle)))
      (set `local.AmountToRemove` (* _quantity (`local.CraftAmount`)))
      (set `self.Remove Item Index in Slots` (`|MakeArray`))
      (bind _output_get (set `local.CurrentItemAmount` 0))
      (set `local.LastSlotItemNumber` _output_get)
      ; 可堆叠物品的移除（多为可消耗材料）
      (bind (_arrayindex _arrayelement) (`/Game/ProjectTD_Old/Blueprints/BlueprintLibrary/BML_MacroForObject.ReverseForEachLoopWithBreak` (`self.Slots`) :!label _label)
        (:`LoopBody`
          (bind (_itemid _quantity_2) (break `/Game/ProjectTD_Old/DataStructure/F_InventorySlot` _arrayelement))
          (if (== (`.RowName` (break `DataTableRowHandle` _itemrowhandle)) _itemid)
            (set `local.CurrentItemAmount` (+ _quantity_2 (`local.CurrentItemAmount`)))
            (`KismetArrayLibrary.Array_Add` (`local.RemoveItemIndexInSlots`) _arrayindex)
            (if (>= _returnvalue 0)
              (set `local.LastSlotItemNumber` _returnvalue)
              (goto _label :!via `Break`))))
        (:`Completed`
          (for (_array_element_2 _array_index) _removeitemindexinslots
            (if (== _array_index (`KismetArrayLibrary.Array_LastIndex` _removeitemindexinslots))
              (if (== 0 _lastslotitemnumber)
                (`KismetArrayLibrary.Array_Set` _slots _array_element_2)
                (else
                  (`KismetArrayLibrary.Array_Set` _slots _array_element_2 (make `/Game/ProjectTD_Old/DataStructure/F_InventorySlot` (`local.CurrentItemID`) _lastslotitemnumber))))
              (else
                (`KismetArrayLibrary.Array_Set` (`self.Slots`) _array_element_2)))))))
    (`self.OnInventoryUpdated`)
    (return (`local.AmountToRemove`))
    (else
      (return 0))))