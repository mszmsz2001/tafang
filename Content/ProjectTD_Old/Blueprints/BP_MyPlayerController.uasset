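; BP_MyPlayerController is a player controller that routes Enhanced Input to the possessed BP_PlayerCharacter.
; BeginPlay adds the IMC_Default mapping context, and possession caches the character as ControlledPawn.
; IA_Move forwards its value to the character's HandleMove for WASD movement.
; IA_Click and IA_Build are empty, and the build menu toggle through ACUIManager is left disconnected, so it never runs.
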(event `self.ReceiveBeginPlay`
  (bind _returnvalue (subsystem `EnhancedInputLocalPlayerSubsystem`))
  ;[1 1 1] 添加输入上下文映射
  (`/Engine/EditorBlueprintResources/StandardMacros.IsValid` _returnvalue
    (:`Is Valid`
      (`EnhancedInputSubsystemInterface.AddMappingContext` _returnvalue "/Game/ProjectTD_Old/Input/IMC_Default.IMC_Default" 0 (struct)))))

(event `EnhancedInput|/Game/ProjectTD_Old/Input/Actions/IA_Move`
  (params (ActionValue :type "Vector2D Structure") (ElapsedSeconds :type "Float (double-precision)") (TriggeredSeconds :type "Float (double-precision)") (InputAction :type "InputAction Object Reference" :default "/Game/ProjectTD_Old/Input/Actions/IA_Move.IA_Move"))
  ;[1 1 1] 角色移动 WASD
  (:`Triggered`
    (`/Game/ProjectTD_Old/Blueprints/BP_PlayerCharacter.HandleMove` (`self.Controlled Pawn`) ActionValue)))

(event `EnhancedInput|/Game/ProjectTD_Old/Input/Actions/IA_Click`
  (params (ActionValue :type Boolean) (ElapsedSeconds :type "Float (double-precision)") (TriggeredSeconds :type "Float (double-precision)") (InputAction :type "InputAction Object Reference" :default "/Game/ProjectTD_Old/Input/Actions/IA_Click.IA_Click")))

(event `EnhancedInput|/Game/ProjectTD_Old/Input/Actions/IA_Build`
  (params (ActionValue :type Boolean) (ElapsedSeconds :type "Float (double-precision)") (TriggeredSeconds :type "Float (double-precision)") (InputAction :type "InputAction Object Reference" :default "/Game/ProjectTD_Old/Input/Actions/IA_Build.IA_Build"))
  ;[1 1 1] 打开/关闭 建造菜单[B]
)

(event `self.ReceivePossess`
  (params (PossessedPawn :type "Pawn Object Reference"))
  (bind _asbp_player_character (cast `/Game/ProjectTD_Old/Blueprints/BP_PlayerCharacter` PossessedPawn))
  (set `self.Controlled Pawn` _asbp_player_character))

(fn `UserConstructionScript`)