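; Base building Blueprint for an interactable station that starts broken, is repaired with materials, then serves as a crafting station.
; A DT_BuildingTable row supplies the mesh, repair cost and unlocked recipes.
; Player contact checks inventory and shows a prompt; interacting drives a timeline progress bar that reverses if interrupted.
; On completion it consumes materials, loads the next-level row and swaps the prompt, after which interaction toggles the crafting menu.
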(event `self.ReceiveBeginPlay`
  (`self.初始化`))

(event `/Game/ProjectTD_Old/Blueprints/Building/BPI_Interactable.主角蓝图引用`
  (params (Player :type "/Game/ProjectTD_Old/Blueprints/BP_PlayerCharacter Object Reference"))
  (if (`self.bIsBroken`)
    _))

(event `/Game/ProjectTD_Old/Blueprints/Building/BPI_Interactable.与物体开始接触`
  (params (Instigator :type "/Game/ProjectTD_Old/Blueprints/BP_PlayerCharacter Object Reference"))
  (bind _output_get (set `self.InstigatorPlayer` Instigator))
  (`self.更新交互信息` _output_get)
  (`self.显示交互信息`))

(event `/Game/ProjectTD_Old/Blueprints/Building/BPI_Interactable.与物体结束接触`
  (params (Instigator :type "/Game/ProjectTD_Old/Blueprints/BP_PlayerCharacter Object Reference"))
  (`|ExecutionSequence`
    (:`then_0`
      (`self.隐藏交互信息`))
    (:`then_1`
      (`self.停止读条修复破损建筑`))))

(event `开始读条修复破损建筑`
  (bind _ac_inventory (`/Game/ProjectTD_Old/Blueprints/BP_PlayerCharacter.AC_Inventory` (`self.InstigatorPlayer`)))
  ; 修复破损建筑
  (if (and (`self.bCanBuild`) (== (`.LevelIndex_29_C550ADC6402E3763AF5920B3CEDDD6B6` (break `/Game/ProjectTD_Old/DataStructure/F_BuildingConfig` (`self.CachedBuildingData`))) 0))
    (bind (_direction _alpha) (`Timeline|RepairBrokenBuilding` :!via `PlayFromStart` :!label _label)
      (:`Update`
        (set `/Game/UI/WBP_RepairWidget.PBarPercent` _alpha (`self.RepairWidget`)))
      (:`Finished`
        (switch `ETimelineDirection` _direction
          (:`Forward`
            (set `self.bIsBroken` false)
            (`/Engine/EditorBlueprintResources/StandardMacros.IsValid` _ac_inventory
              (:`Is Valid`
                (`/Game/ProjectTD_Old/Blueprints/ActorComponent/AC_Inventory.移除物品（消耗材料）` _ac_inventory true (`.UpgradeCost_49_58FC28D3433E71B7F29DCCB07C878B54` (break `/Game/ProjectTD_Old/DataStructure/F_BuildingConfig` (`self.CachedBuildingData`))) 1)
                (`self.升级建筑`)
                (`self.更换为建筑功能交互面板`)
                (`self.更新制造面板`)))))))))

(event `/Game/ProjectTD_Old/Blueprints/Building/BPI_Interactable.交互开始`
  (params (Instigator :type "/Game/ProjectTD_Old/Blueprints/BP_PlayerCharacter Object Reference"))
  (set `self.InstigatorPlayer` Instigator)
  (if (`self.bIsBroken`)
    (`self.开始读条修复破损建筑`)
    (elif (`self.bIsOpenStationMenu`)
      (`self.关闭制造面板`)
      (set `self.bIsOpenStationMenu` false)
      (else
        (`self.打开制造面板`)
        (set `self.bIsOpenStationMenu` true)))))

(event `停止读条修复破损建筑`
  ; 修复破损建筑
  (if (and (`self.bCanBuild`) (== (`.LevelIndex_29_C550ADC6402E3763AF5920B3CEDDD6B6` (break `/Game/ProjectTD_Old/DataStructure/F_BuildingConfig` (`self.CachedBuildingData`))) 0))
    (goto _label :!via `Reverse`)))

(event `/Game/ProjectTD_Old/Blueprints/Building/BPI_Interactable.交互结束`
  (params (Instigator :type "/Game/ProjectTD_Old/Blueprints/BP_PlayerCharacter Object Reference"))
  (set `self.InstigatorPlayer` Instigator)
  (if (`self.bIsBroken`)
    (`self.停止读条修复破损建筑`)))

(fn `UserConstructionScript`)

(fn `关闭制造面板`
  (`Widget.RemoveFromParent` (`self.StationMenuRef`)))

(fn `初始化`
  (bind _returnvalue (`|GetDataTableRow` "/Game/ProjectTD_Old/DataStructure/DT_BuildingTable.DT_BuildingTable" (`self.CurrentRowID`))
    (:`then`
      (set `self.CachedBuildingData` _returnvalue)
      (`self.更换模型`)
      (`|ExecutionSequence`
        (:`then_0`
          ;[1 1 1] 交互UI
          (bind _aswbp_repair_widget (cast `/Game/UI/WBP_RepairWidget` (`WidgetComponent.GetUserWidgetObject` (`self.PromptWidget`))))
          (set `self.RepairWidget` _aswbp_repair_widget)
          (bind _returnvalue_2 (`|CreateWidget` "/Game/UI/WBP_OpenMenu.WBP_OpenMenu_C" (`GameplayStatics.GetPlayerController` 0))) ; 必须有这一步，不然给PromptWidget赋值会出错，因为CommonUI要指定playercontroller
          (set `self.OpenWidget` _returnvalue_2))
        (:`then_1`
          ;[1 1 1] 工作台页面UI
          (bind _returnvalue_3 (`|CreateWidget` "/Game/UI/WBP_Station_Main.WBP_Station_Main_C" (`GameplayStatics.GetPlayerController` 0) (`.UnlockedRecipes_42_002498B34B06CC3A4133DCB9E570CB30` (break `/Game/ProjectTD_Old/DataStructure/F_BuildingConfig` (`self.CachedBuildingData`)))))
          (set `self.StationMenuRef` _returnvalue_3))
        (:`then_3`
          (return))))
    (:`RowNotFound`
      (`KismetSystemLibrary.PrintString` "未找到建筑ID"))))

(fn `升级建筑`
  ;[1 1 1] 设置建筑升级后的数据（下一个数据）
  (bind _output_get (set `self.CurrentRowID` (`.NextLevelID_35_82916F394C932E8854C8F8AC5171E11E` (break `/Game/ProjectTD_Old/DataStructure/F_BuildingConfig` (`self.CachedBuildingData`)))))
  (bind _returnvalue (`|GetDataTableRow` "/Game/ProjectTD_Old/DataStructure/DT_BuildingTable.DT_BuildingTable" _output_get)
    (:`then`
      (set `self.CachedBuildingData` _returnvalue)
      (set `self.CurrentLevel` 1)
      (`self.更换模型`))))

(fn `打开制造面板`
  (bind _stationmenuref (`self.StationMenuRef`))
  (set `/Game/UI/WBP_Station_Main.AC_InventoryRef` (`/Game/ProjectTD_Old/Blueprints/BP_PlayerCharacter.AC_Inventory` (`self.InstigatorPlayer`)) _stationmenuref)
  (`UserWidget.AddToViewport` _stationmenuref 0))

(fn `显示交互信息`
  (`SceneComponent.SetVisibility` (`self.PromptWidget`) true false))

(fn `更换为建筑功能交互面板`
  (bind _openwidget (`self.OpenWidget`))
  (`WidgetComponent.SetWidget` (`self.PromptWidget`) _openwidget)
  (`KismetSystemLibrary.PrintString` (`KismetSystemLibrary.GetDisplayName` _openwidget)))

(fn `更换模型`
  (`StaticMeshComponent.SetStaticMesh` (`self.StaticMesh`) (`.BuildingMesh_47_1015877B49C5652C35B6089BBE56A7AC` (break `/Game/ProjectTD_Old/DataStructure/F_BuildingConfig` (`self.CachedBuildingData`))))
  (return))

(fn `更新交互信息`
  (params (`目标` :type "/Game/ProjectTD_Old/Blueprints/BP_PlayerCharacter Object Reference"))
  (bind _ac_inventory (`/Game/ProjectTD_Old/Blueprints/BP_PlayerCharacter.AC_Inventory` `目标`))
  (set `/Game/UI/WBP_RepairWidget.AC_InventoryRef` _ac_inventory (`self.RepairWidget`))
  (bind _upgradecostarray (`self.获取消耗材料数组`))
  (bind _bcanremove (`/Game/ProjectTD_Old/Blueprints/ActorComponent/AC_Inventory.判断材料是否足够消耗` _ac_inventory _upgradecostarray))
  (bind _output_get (set `self.bCanBuild` _bcanremove))
  (`/Game/UI/WBP_RepairWidget.刷新面板信息` (`self.RepairWidget`) _output_get _upgradecostarray))

(fn `更新制造面板`
  (set `/Game/UI/WBP_Station_Main.UnlockRecipes` (`.UnlockedRecipes_42_002498B34B06CC3A4133DCB9E570CB30` (break `/Game/ProjectTD_Old/DataStructure/F_BuildingConfig` (`self.CachedBuildingData`))) (`self.StationMenuRef`))
  (return))

(fn `获取消耗材料数组`
  (returns (UpgradeCostArray :type "Array of /Game/ProjectTD_Old/DataStructure/F_CostItem Structure"))
  (return (`.UpgradeCost_49_58FC28D3433E71B7F29DCCB07C878B54` (break `/Game/ProjectTD_Old/DataStructure/F_BuildingConfig` (`self.CachedBuildingData`)))))

(fn `隐藏交互信息`
  (`SceneComponent.SetVisibility` (`self.PromptWidget`) false false))