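; BP_BuildPlane is a grid plane actor, apparently a build area, sized by an integer GridSize.
; Its construction script calls SetupGridParameters, which keeps each GridSize axis at 1 or above and stores the product as CellCount.
; The same function scales GridMesh in X and Y to the grid dimensions, one scale unit per cell.
; The event graph holds only disabled placeholder events, so it has no runtime logic.
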(fn `SetupGridParameters`
  (bind (_x _y) (break `IntPoint` (`self.GridSize`)))
  (bind (_x_2 _y_2) (break `IntPoint` (`self.GridSize`)))
  (bind (_x_3 _y_3) (break `IntPoint` (`self.GridSize`)))
  (set `self.GridSize` (make `IntPoint` (`KismetMathLibrary.Clamp` _x_2 1 _x_2) (`KismetMathLibrary.Clamp` _y_2 1 _y_2)))
  (set `self.CellCount` (* _x_3 _y_3))
  (`SceneComponent.SetRelativeScale3D` (`self.GridMesh`) (`KismetMathLibrary.MakeVector` (`KismetMathLibrary.Conv_IntToDouble` _x) (`KismetMathLibrary.Conv_IntToDouble` _y) 1.0)))

(fn `UserConstructionScript`
  (`self.SetupGridParameters`))