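; BP_Bullet is a weapon projectile actor that flies by ProjectileMovement, with its speed and range taken from weapon data.
; UpdateBulletData stores Range and BulletSpeed, then multiplies the current velocity by BulletSpeed.
; The custom event 销毁 (Destroy) waits Range / BulletSpeed seconds before destroying the actor; nothing in this graph calls it.
; No hit or damage logic exists here, as the overlap event is disabled.
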(event `self.ReceiveBeginPlay`)

(event `销毁`
  (`KismetSystemLibrary.Delay` (/ (`self.Range`) (`self.Bullet Speed`)))
  (`self.K2_DestroyActor`))

(fn `UpdateBulletData`
  (params (WeaponData :type "/Game/ProjectTD_Old/DataStructure/DataAsset/BP_WeaponDataAsset Object Reference"))
  (set `self.Range` (`/Game/ProjectTD_Old/DataStructure/DataAsset/BP_WeaponDataAsset.Range` WeaponData))
  (set `self.Bullet Speed` (`/Game/ProjectTD_Old/DataStructure/DataAsset/BP_WeaponDataAsset.BulletSpeed` WeaponData))
  (set `MovementComponent.Velocity` (* (`self.GetVelocity`) (`self.Bullet Speed`)) (`self.ProjectileMovement`)))

(fn `UserConstructionScript`)