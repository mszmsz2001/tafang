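; BP_VS_HUD is the player HUD Blueprint that creates and shows or hides the main HUD, pause menu, inventory screen and action menu widgets.
; On BeginPlay it builds each widget from a template through a pool that reuses instances by class, with only the HUD shown.
; Wrapper functions toggle, show or hide each widget by adding it to or removing it from the viewport, with the action menu also positioned on screen.
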(event `self.ReceiveBeginPlay`
  ; Spawn HUD Widget
  (bind _return_widget (`self.Add New Widget` (`self.HUD Template`) "NewEnumerator0"))
  (set `self.HUD Widget` _return_widget)
  (bind _return_widget_2 (`self.Add New Widget` (`self.Pause Menu Template`) "NewEnumerator1"))
  (set `self.Pause Menu Widget` _return_widget_2)
  (bind _return_widget_3 (`self.Add New Widget` (`self.Inventory Screen Template`) "NewEnumerator1"))
  (set `self.Inventory Screen Widget` _return_widget_3)
  (bind _return_widget_4 (`self.Add New Widget` (`self.Action Menu Template`) "NewEnumerator1"))
  (set `self.Action Menu` _return_widget_4))

(fn `Add New Widget`
  (params (WidgetTemplate :type "UserWidget Class Reference") (`Default Visibility` :type "/Game/VisualSandbox/Blueprints/Enumerations/EWidgetVisibility Enum" :default "NewEnumerator3"))
  (returns (`Return Widget` :type "UserWidget Object Reference"))
  (locals (`Widget Found` :type "UserWidget Object Reference"))
  (bind (_widget_found _successful) (`self.Find Widget By Class` (`local.WidgetTemplate`)))
  (`local.WidgetTemplate`
    (:`then`
      (`|ExecutionSequence`
        (:`then_0`
          ; Search for widget template
          (set `local.Widget Found` _widget_found)
          (if (not _successful)
            ; Create brand new widget and add to HUD Widget Pool
            (bind _returnvalue (`|CreateWidget` (`local.WidgetTemplate`) (`self.GetOwningPlayerController`)))
            (bind _output_get (set `local.Widget Found` _returnvalue))
            (`KismetArrayLibrary.Array_AddUnique` (`self.HUD Widget Pool`) _output_get)))
        (:`then_1`
          ; Set Widget Visibility
          (`self.Set Widget Visibility` (`local.Widget Found`) (`local.Default Visibility`))
          (return (`local.Widget Found`)))))
    (:`else`)))

(fn `Find Widget By Class`
  (params (`Widget Class` :type "UserWidget Class Reference"))
  (returns (`Widget Found` :type "UserWidget Object Reference") (Successful :type Boolean))
  (locals (W :type "UserWidget Object Reference"))
  ; Loop body HUD Widgets pool
  (for _array_element (`self.HUD Widget Pool`)
    (bind _output_get (set `local.W` _array_element))
    (`/Engine/EditorBlueprintResources/StandardMacros.IsValid` _output_get
      (:`Is Valid`
        ; Checks widget class
        (if (== (`GameplayStatics.GetObjectClass` (`local.W`)) (`local.Widget Class`))
          (return (`local.W`) true))))))

(fn `Get HUD Widget`
  (returns (`Return HUD Widget` :type "UserWidget Object Reference"))
  (return (`self.HUD Widget`)))

(fn `Set Action Menu Visibility`
  (params (`New Visibility` :type "/Game/VisualSandbox/Blueprints/Enumerations/EWidgetVisibility Enum" :default "NewEnumerator3") (`Display Position` :type "Vector2D Structure"))
  (returns (`Return Visible` :type Boolean) (`Action Menu Widget` :type "UserWidget Object Reference"))
  (bind _action_menu (`self.Action Menu`)
    (:`then`
      (bind _return_visible (`self.Set Widget Visibility` _action_menu (`local.New Visibility`)))
      (`|ExecutionSequence`
        (:`then_0`
          (`UserWidget.SetPositionInViewport` (`self.Action Menu`) (`local.Display Position`) true))
        (:`then_1`
          (return _return_visible (`self.Action Menu`)))))
    (:`else`)))

(fn `Set HUD Visibility`
  (params (`New Visibility` :type "/Game/VisualSandbox/Blueprints/Enumerations/EWidgetVisibility Enum" :default "NewEnumerator3"))
  (returns (Successful :type Boolean))
  (bind _return_visible (`self.Set Widget Visibility` (`self.HUD Widget`) (`local.New Visibility`)))
  (`|ExecutionSequence`
    (:`then_0`
      (`self.Set Action Menu Visibility` "NewEnumerator1"))
    (:`then_1`
      (return _return_visible))))

(fn `Set Inventory Screen Visibility`
  (params (`New Visibility` :type "/Game/VisualSandbox/Blueprints/Enumerations/EWidgetVisibility Enum" :default "NewEnumerator3"))
  (returns (`Return Visible` :type Boolean) (`Inventory Widget` :type "UserWidget Object Reference"))
  (bind _return_visible (`self.Set Widget Visibility` (`self.Inventory Screen Widget`) (`local.New Visibility`)))
  (return _return_visible (`self.Inventory Screen Widget`)))

(fn `Set Pause Menu Visibility`
  (params (`New Visibility` :type "/Game/VisualSandbox/Blueprints/Enumerations/EWidgetVisibility Enum" :default "NewEnumerator3"))
  (returns (`Return Visible` :type Boolean))
  (bind _return_visible (`self.Set Widget Visibility` (`self.Pause Menu Widget`) (`local.New Visibility`)))
  (return _return_visible))

(fn `Set Widget Visibility`
  (params (`Widget Target` :type "UserWidget Object Reference") (`New Visibility` :type "/Game/VisualSandbox/Blueprints/Enumerations/EWidgetVisibility Enum" :default "NewEnumerator3"))
  (returns (`Return Visible` :type Boolean))
  (bind _widget_target (`local.Widget Target`))
  (bind _returnvalue (`Widget.IsVisible` (`local.Widget Target`)))
  (`/Engine/EditorBlueprintResources/StandardMacros.IsValid` `Widget Target`
    (:`Is Valid`
      (`|ExecutionSequence`
        (:`then_0`
          ; switch widget visibility
          (switch `/Game/VisualSandbox/Blueprints/Enumerations/EWidgetVisibility` (`local.New Visibility`)
            (:`NewEnumerator3`
              (if _returnvalue
                (`Widget.RemoveFromParent` _widget_target)
                (else
                  (`UserWidget.AddToViewport` _widget_target 0))))
            (:`NewEnumerator0`
              (if (not _returnvalue)
                (`UserWidget.AddToViewport` _widget_target 0)))
            (:`NewEnumerator1`
              (if _returnvalue
                (`Widget.RemoveFromParent` _widget_target)))))
        (:`then_1`
          (return (`Widget.IsVisible` (`local.Widget Target`))))))))

(fn `UserConstructionScript`)