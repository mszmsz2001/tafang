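; Player character that aims at the mouse cursor, shoots, interacts with objects and manages an inventory and HUD.
; Weapon inputs toggle a spawned pistol or rifle attached to mesh sockets; its data asset drives montages, bullets, fire interval and reloads from inventory ammo.
; Rifles also fire while held, gated by a delay.
; A forward overlap component sets the interface-driven interaction target, and debug keys test HP/MP and items.
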(event OnComponentBeginOverlap(InteractDetectForward)
  (params (OverlappedComponent :type Primitive%20Component%20Object%20Reference) (OtherActor :type Actor%20Object%20Reference) (OtherComp :type Primitive%20Component%20Object%20Reference) (OtherBodyIndex :type Integer) (bFromSweep :type Boolean) (SweepResult :type Hit%20Result%20Structure%20%28by%20ref%29))
  ;[0.15 0.15 0.15 0.5] 接触建筑物体并交互
  (Class|BPIInteractable|与物体开始接触(Message) OtherActor self)
  (bind _output_get (Variables|Default|SetCurrentInteractTarget OtherActor))
  (bind _upgradecostarray (Class|BPIInteractable|获取消耗材料数组(Message) _output_get))
  (for _array_element _upgradecostarray
    _))

(event OnComponentEndOverlap(InteractDetectForward)
  (params (OverlappedComponent :type Primitive%20Component%20Object%20Reference) (OtherActor :type Actor%20Object%20Reference) (OtherComp :type Primitive%20Component%20Object%20Reference) (OtherBodyIndex :type Integer))
  ;[0.15 0.15 0.15 0.5] 接触建筑物体并交互
  (Class|BPIInteractable|与物体结束接触(Message) OtherActor self)
  (Variables|Default|SetCurrentInteractTarget 0))

(event EventBeginPlay
  (bind _returnvalue (PlayerController|LocalPlayerSubsystems|GetEnhancedInputLocalPlayerSubsystem))
  ;[1 1 1] 添加输入上下文映射
  (Utilities|IsValid _returnvalue
    (:Is%20Valid
      (Input|AddMappingContext _returnvalue "/Game/ProjectTD/Input/IMC_Default.IMC_Default" 0 "(bIgnoreAllPressedKeysUntilRelease=True,bForceImmediately=False,bNotifyUserSettings=False)")
      (Variables|/Script/Engine.PlayerController|SetbShowMouseCursor (Game|GetPlayerController 0) true)
      (bind _returnvalue_2 (UserInterface|CreateWidget "/Game/UI/WBP_HPMP_HUD.WBP_HPMP_HUD_C"))
      (Variables|Default|SetHUD_HPMP _returnvalue_2)
      (UserInterface|Viewport|AddtoViewport _returnvalue_2 0)
      (CallFunction|UIFirstUpdateHPMP))))

(event Collision|EventActorBeginOverlap
  (params (OtherActor :type Actor%20Object%20Reference)))

(event EventTick
  (params (DeltaSeconds :type Float%20%28single-precision%29))
  (|将角色朝向光标位置))

(event Input|MouseEvents|LeftMouseButton
  (params (Key :type Key%20Structure :default "None"))
  (:Pressed
    (Animation|PlayAnimMontage 0 1.0 "None")))

(event Input|KeyboardEvents|Q
  (params (Key :type Key%20Structure :default "None")))

(event Input|KeyboardEvents|Q
  (params (Key :type Key%20Structure :default "None"))
  (:Released
    (bind _output_get (Variables|HP|SetCurrentHP (- (Variables|HP|GetCurrentHP) 5.0)))
    (CallFunction|UIUpdateHP _output_get 1e+02)))

(event Input|KeyboardEvents|E
  (params (Key :type Key%20Structure :default "None"))
  (:Released
    (bind _output_get (Variables|MP|SetCurrentMP (+ (Variables|MP|GetCurrentMP) 5.0)))
    (CallFunction|UIUpdateMP _output_get 1e+02)))

(event Input|EnhancedActionEvents|EnhancedInputActionIA_Interact
  (params (ActionValue :type Boolean) (ElapsedSeconds :type Float%20%28double-precision%29) (TriggeredSeconds :type Float%20%28double-precision%29) (InputAction :type Input%20Action%20Object%20Reference :default "/Game/ProjectTD/Input/Actions/IA_Interact.IA_Interact"))
  (bind _self self)
  (bind _currentinteracttarget (Variables|Default|GetCurrentInteractTarget))
  (bind _currentinteracttarget_2 (Variables|Default|GetCurrentInteractTarget))
  ;[0.15 0.15 0.15 0.5] [E]键-交互
  (:Started
    (Utilities|IsValid _currentinteracttarget_2
      (:Is%20Valid
        (Class|BPIInteractable|交互开始(Message) _currentinteracttarget_2 _self))))
  (:Completed
    (Utilities|IsValid _currentinteracttarget
      (:Is%20Valid
        (Class|BPIInteractable|交互结束(Message) _currentinteracttarget _self)))))

(event Input|EnhancedActionEvents|EnhancedInputActionIA_OpenBag
  (params (ActionValue :type Boolean) (ElapsedSeconds :type Float%20%28double-precision%29) (TriggeredSeconds :type Float%20%28double-precision%29) (InputAction :type Input%20Action%20Object%20Reference :default "/Game/ProjectTD/Input/Actions/IA_OpenBag.IA_OpenBag"))
  (bind _ac_inventory (Variables|Default|GetAC_Inventory))
  ;[0.15 0.15 0.15 0.5] 按[B]键-打开背包
  (:Completed
    (if (Variables|Default|GetbUseBag)
      (Default|关闭背包 _ac_inventory)
      (Variables|Default|SetbUseBag false)
      (else
        (Default|打开背包 _ac_inventory)
        (Variables|Default|SetbUseBag true)))))

(event Input|EnhancedActionEvents|EnhancedInputActionIA_weapon1
  (params (ActionValue :type Boolean) (ElapsedSeconds :type Float%20%28double-precision%29) (TriggeredSeconds :type Float%20%28double-precision%29) (InputAction :type Input%20Action%20Object%20Reference :default "/Game/ProjectTD/Input/Actions/IA_weapon1.IA_weapon1"))
  ;[1 1 1] 按1切换手枪
  (:Canceled
    (if (Variables|Default|Getpistol_armed) :!label _label
      ;;[0.15 0.15 0.15 0.5] 如果当前已经装备了步枪，就放下步枪。rifle_armed是切换动画为无步枪动画。后面是为了摧毁当前装备武器的actor
      (Variables|Default|Setpistol_armed false)
      (Utilities|IsValid (Variables|Default|GetCurrent_Weapon)
        (:Is%20Valid
          (Actor|DestroyActor (Variables|Default|GetCurrent_Weapon))))
      (else
        (Utilities|FlowControl|Sequence
          (:then_0
            ;;[0.15 0.15 0.15 0.5] 如果没装备，装备上步枪，这里是为了切换动画状态
            (Variables|Default|Setrifle_armed false)
            (Variables|Default|Setpistol_armed true))
          (:then_1
            ;;[0.15 0.15 0.15 0.5] 先摧毁当前装备的武器, 然后把武器附加到角色骨骼上
            (Utilities|IsValid (Variables|Default|GetCurrent_Weapon)
              (:Is%20Valid
                (Actor|DestroyActor (Variables|Default|GetCurrent_Weapon)))
              (:Is%20Not%20Valid
                _))
            (bind _returnvalue (Game|SpawnActorfromClass "/Game/ProjectTD/Blueprints/Weapon/BP_Weapon_Pistol_01.BP_Weapon_Pistol_01_C" (Transformation|GetActorTransform) "Undefined" "MultiplyWithRoot" 0 0))
            (bind _output_get (Variables|Default|SetCurrent_Weapon _returnvalue))
            (Variables|Default|SetData%20Asset (Variables|/Game/ProjectTD/Blueprints/Weapon/BP_Weapon_Pistol_01.BP_Weapon_Pistol_01_C|GetData_asset _returnvalue))
            (Transformation|AttachComponentToComponent (Variables|/Script/Engine.Actor|GetRootComponent _output_get) (Variables|Character|GetMesh) "Pistol" "SnapToTarget" "SnapToTarget" "SnapToTarget" true)
            (CallFunction|UIUpdateBullet))))))
  (:Completed
    (goto _label)))

(event Input|EnhancedActionEvents|EnhancedInputActionIA_weapon2
  (params (ActionValue :type Boolean) (ElapsedSeconds :type Float%20%28double-precision%29) (TriggeredSeconds :type Float%20%28double-precision%29) (InputAction :type Input%20Action%20Object%20Reference :default "/Game/ProjectTD/Input/Actions/IA_weapon2.IA_weapon2"))
  ;[1 1 1] 按2切换步枪
  (:Canceled
    (if (Variables|Default|Getrifle_armed) :!label _label
      ;;[0.15 0.15 0.15 0.5] 如果当前已经装备了步枪，就放下步枪。rifle_armed是切换动画为无步枪动画。后面是为了摧毁当前装备武器的actor
      (Variables|Default|Setrifle_armed false)
      (Utilities|IsValid (Variables|Default|GetCurrent_Weapon)
        (:Is%20Valid
          (Actor|DestroyActor (Variables|Default|GetCurrent_Weapon))))
      (else
        (Utilities|FlowControl|Sequence
          (:then_0
            ;;[0.15 0.15 0.15 0.5] 如果没装备，装备上步枪，这里是为了切换动画状态
            (Variables|Default|Setpistol_armed false)
            (Variables|Default|Setrifle_armed true))
          (:then_1
            ;;[0.15 0.15 0.15 0.5] 先摧毁当前装备的武器, 然后把武器附加到角色骨骼上
            (Utilities|IsValid (Variables|Default|GetCurrent_Weapon)
              (:Is%20Valid
                (Actor|DestroyActor (Variables|Default|GetCurrent_Weapon)))
              (:Is%20Not%20Valid
                _))
            (bind _returnvalue (Game|SpawnActorfromClass "/Game/ProjectTD/Blueprints/Weapon/BP_Weapon_Rifle_01.BP_Weapon_Rifle_01_C" (Transformation|GetActorTransform) "Undefined" "MultiplyWithRoot" 0 0))
            (bind _output_get (Variables|Default|SetCurrent_Weapon _returnvalue))
            (Variables|Default|SetData%20Asset (Variables|/Game/ProjectTD/Blueprints/Weapon/BP_Weapon_Rifle_01.BP_Weapon_Rifle_01_C|GetData_asset _returnvalue))
            (Transformation|AttachComponentToComponent (Variables|/Script/Engine.Actor|GetRootComponent _output_get) (Variables|Character|GetMesh) "Rifle" "SnapToTarget" "SnapToTarget" "SnapToTarget" true)
            (CallFunction|UIUpdateBullet))))))
  (:Completed
    (goto _label)))

(event Input|EnhancedActionEvents|EnhancedInputActionIA_Click
  (params (ActionValue :type Boolean) (ElapsedSeconds :type Float%20%28double-precision%29) (TriggeredSeconds :type Float%20%28double-precision%29) (InputAction :type Input%20Action%20Object%20Reference :default "/Game/ProjectTD/Input/Actions/IA_Click.IA_Click"))
  (bind _pistol_armed (Variables|Default|Getpistol_armed))
  (bind _rifle_armed (Variables|Default|Getrifle_armed))
  (bind _returnvalue (or _pistol_armed _rifle_armed))
  ;[0.15 0.15 0.15 0.5] 开火逻辑,手枪仅能点按(started)    步枪点按和持续按压都可以
  (:Triggered
    ;;[0.15 0.15 0.15 0.5] 只有装备了武器才能开火
    (if _returnvalue
      ;;[0.15 0.15 0.15 0.5] 持续开火只有步枪才可以，所以这里的triigger判断下是否为步枪
      (switch Utilities|FlowControl|Switch|SwitchonWeapon_type (Variables|/Game/ProjectTD/结构与枚举/DataAsset/BP_WeaponDataAsset.BP_WeaponDataAsset_C|Getweapon_type (Variables|Default|GetData%20Asset))
        (:NewEnumerator1
          (if (== (Variables|Default|GetCurrenBullet) 0) :!label _label
            (CallFunction|补充子弹)
            (else
              (|开火逻辑)))))))
  (:Started
    (if _returnvalue
      (goto _label))))

(event Input|KeyboardEvents|DebugKeyR
  (params (Key :type Key%20Structure :default "None") (ActionValue :type Input%20Action%20Value%20Structure))
  (:Pressed
    (if (< (Variables|Default|GetCurrenBullet) (Variables|/Game/ProjectTD/结构与枚举/DataAsset/BP_WeaponDataAsset.BP_WeaponDataAsset_C|GetBulletStorage (Variables|Default|GetData%20Asset)))
      (CallFunction|补充子弹)
      (CallFunction|UIUpdateBullet))))

(event Input|KeyboardEvents|DebugKeyF
  (params (Key :type Key%20Structure :default "None") (ActionValue :type Input%20Action%20Value%20Structure))
  (bind _ac_inventory (Variables|Default|GetAC_Inventory))
  (bind _slots (Variables|/Game/ProjectTD/Blueprints/ActorComponent/AC_Inventory.AC_Inventory_C|GetSlots _ac_inventory))
  ;[0.15 0.15 0.15 0.5] Debug
  (:Pressed
    (Development|PrintString (Utilities|String|ToString(Integer) (.quantity (Utilities|Array|Get(acopy) _slots))))
    (Development|PrintString (Utilities|String|ToString(Integer) (.quantity (Utilities|Array|Get(acopy) _slots 1))))))

(event Input|KeyboardEvents|DebugKeyT
  (params (Key :type Key%20Structure :default "None") (ActionValue :type Input%20Action%20Value%20Structure))
  ;[0.15 0.15 0.15 0.5] Debug
  (:Pressed
    (Default|添加物品 (Variables|Default|GetAC_Inventory) "Mat_Wood" 10 0.0)
    (Default|添加物品 (Variables|Default|GetAC_Inventory) "Bullet_01" 10 0.0)
    (Default|添加物品 (Variables|Default|GetAC_Inventory) "Bullet_02" 10 0.0)
    (CallFunction|UIUpdateBullet)))

(event Input|KeyboardEvents|DebugKeyX
  (params (Key :type Key%20Structure :default "None") (ActionValue :type Input%20Action%20Value%20Structure))
  (bind _ac_inventory (Variables|Default|GetAC_Inventory))
  ;[0.15 0.15 0.15 0.5] Debug
  (:Pressed
    (bind (_bcanremove _outitemarray) (Default|判断材料是否足够消耗 _ac_inventory (Utilities|Array|MakeArray (Utilities|Struct|MakeF_CostItem (Utilities|Struct|MakeDataTableRowHandle "/Game/ProjectTD/结构与枚举/DT_Item.DT_Item" "Mat_Wood") 5))))
    (Default|移除物品（消耗材料） _ac_inventory _bcanremove _outitemarray 1)))

(fn ConstructionScript)

(fn HandleMove
  (params (Direction :type Vector%202D%20Structure))
  (Pawn|Input|AddMovementInput "1.000000,0.000000,0.000000" (.x Direction) false)
  (Pawn|Input|AddMovementInput "0.000000,1.000000,0.000000" (.y Direction) false))

(fn Fire
  (bind _data_asset (Variables|Default|GetData%20Asset))
  (bind _animationmontage (Variables|/Game/ProjectTD/结构与枚举/DataAsset/BP_WeaponDataAsset.BP_WeaponDataAsset_C|GetAnimationMontage _data_asset))
  (Animation|PlayAnimMontage _animationmontage 1.0 "None")
  (Development|PrintString (Utilities|GetDisplayName _animationmontage)))

(fn UIFirstUpdateHPMP
  (bind _self self)
  (bind _self_2 self)
  (bind _hud_hpmp (Variables|Default|GetHUD_HPMP _self_2))
  (bind _hud_hpmp_2 (Variables|Default|GetHUD_HPMP _self))
  (Class|BIHPMP|UpdatePlayerCurrentHP(Message) _hud_hpmp_2 (Variables|HP|GetCurrentHP))
  (Class|BIHPMP|UpdatePlayerHPBarPercent(Message) _hud_hpmp_2 (/ (Variables|HP|GetCurrentHP) (Variables|HP|GetMaxHP)))
  (Class|BIHPMP|UpdatePlayerMaxHP(Message) _hud_hpmp_2 (Variables|HP|GetMaxHP))
  (Class|BIHPMP|UpdatePlayerMaxMP(Message) _hud_hpmp (Variables|MP|GetMaxMP))
  (Class|BIHPMP|UpdatePlayerCurrentMP(Message) _hud_hpmp (/ (Variables|MP|GetCurrentMP) (Variables|MP|GetMaxMP)))
  (Class|BIHPMP|UpdatePlayerMPBarPercent(Message) _hud_hpmp (Variables|MP|GetCurrentMP)))

(fn UIUpdateHP
  (params (CurrentHP :type Float%20%28double-precision%29) (MaxHP :type Float%20%28double-precision%29))
  (bind _self self)
  (bind _hud_hpmp (Variables|Default|GetHUD_HPMP _self))
  (Class|BIHPMP|UpdatePlayerCurrentHP(Message) _hud_hpmp CurrentHP)
  (Class|BIHPMP|UpdatePlayerHPBarPercent(Message) _hud_hpmp (/ CurrentHP MaxHP))
  (Class|BIHPMP|UpdatePlayerMaxHP(Message) _hud_hpmp MaxHP))

(fn UIUpdateMP
  (params (CurrentMP :type Float%20%28double-precision%29) (MaxMP :type Float%20%28double-precision%29))
  (bind _self self)
  (bind _hud_hpmp (Variables|Default|GetHUD_HPMP _self))
  (Class|BIHPMP|UpdatePlayerMaxMP(Message) _hud_hpmp MaxMP)
  (Class|BIHPMP|UpdatePlayerCurrentMP(Message) _hud_hpmp CurrentMP)
  (Class|BIHPMP|UpdatePlayerMPBarPercent(Message) _hud_hpmp (/ CurrentMP MaxMP)))

(fn 补充子弹
  (bind _data_asset (Variables|Default|GetData%20Asset))
  (bind _ammotypeid (Variables|/Game/ProjectTD/结构与枚举/DataAsset/BP_WeaponDataAsset.BP_WeaponDataAsset_C|GetAmmoTypeID _data_asset))
  (bind _outitemamount (Default|查询物品数量 (Variables|Default|GetAC_Inventory) (Variables|/Game/ProjectTD/结构与枚举/DataAsset/BP_WeaponDataAsset.BP_WeaponDataAsset_C|GetAmmoTypeID (Variables|Default|GetData%20Asset))))
  (if (> _outitemamount 0)
    (Animation|PlayAnimMontage (Variables|/Game/ProjectTD/结构与枚举/DataAsset/BP_WeaponDataAsset.BP_WeaponDataAsset_C|GetReloadMontage (Variables|Default|GetData%20Asset)) 1.0 "None")
    (bind _outitemamount_2 (Default|查询物品数量 (Variables|Default|GetAC_Inventory) _ammotypeid))
    (if (>= _outitemamount_2 (- (Variables|/Game/ProjectTD/结构与枚举/DataAsset/BP_WeaponDataAsset.BP_WeaponDataAsset_C|GetBulletStorage (Variables|Default|GetData%20Asset)) (Variables|Default|GetCurrenBullet)))
      (Default|移除物品（消耗材料） (Variables|Default|GetAC_Inventory) true (Utilities|Array|MakeArray (Utilities|Struct|MakeF_CostItem (Utilities|Struct|MakeDataTableRowHandle "/Game/ProjectTD/结构与枚举/DT_Item.DT_Item" _ammotypeid) (- (Variables|/Game/ProjectTD/结构与枚举/DataAsset/BP_WeaponDataAsset.BP_WeaponDataAsset_C|GetBulletStorage (Variables|Default|GetData%20Asset)) (Variables|Default|GetCurrenBullet)))) 1)
      (Variables|Default|SetCurrenBullet (Variables|/Game/ProjectTD/结构与枚举/DataAsset/BP_WeaponDataAsset.BP_WeaponDataAsset_C|GetBulletStorage (Variables|Default|GetData%20Asset)))
      (else
        (Default|移除物品（消耗材料） (Variables|Default|GetAC_Inventory) true (Utilities|Array|MakeArray (Utilities|Struct|MakeF_CostItem (Utilities|Struct|MakeDataTableRowHandle "/Game/ProjectTD/结构与枚举/DT_Item.DT_Item" _ammotypeid) _outitemamount_2)) 1)
        (Variables|Default|SetCurrenBullet (+ (Variables|Default|GetCurrenBullet) _outitemamount_2))))))

(fn UIUpdateBullet
  (bind _outitemamount (Default|查询物品数量 (Variables|Default|GetAC_Inventory) (Variables|/Game/ProjectTD/结构与枚举/DataAsset/BP_WeaponDataAsset.BP_WeaponDataAsset_C|GetAmmoTypeID (Variables|Default|GetData%20Asset))))
  (Class|BIHPMP|UpdateBullet(Message) (Variables|Default|GetHUD_HPMP self) (Variables|Default|GetCurrenBullet) _outitemamount))