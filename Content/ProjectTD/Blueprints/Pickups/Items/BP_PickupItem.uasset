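; World pickup item that the player can collect into an inventory by interacting with it.
; On BeginPlay it looks up its ItemID in DT_Item to set the drop mesh and display name, which it exposes with the quantity as interaction info.
; The Sensor overlap registers it as an interactable on BP_ThirdPerson_Pawn, and contact events toggle the prompt widget.
; Interaction tries adding the item, then destroys the actor or prints a bag-full message.
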(event `self.ReceiveBeginPlay`
  (`self.初始化`))

(event `self.Sensor.OnComponentBeginOverlap`
  (params (OverlappedComponent :type "PrimitiveComponent Object Reference") (OtherActor :type "Actor Object Reference") (OtherComp :type "PrimitiveComponent Object Reference") (OtherBodyIndex :type Integer) (bFromSweep :type Boolean) (SweepResult :type "HitResult Structure (by ref)"))
  (bind _asbp_third_person_pawn (cast `/Game/ProjectTD/Blueprints/Player/BP_ThirdPerson_Pawn` OtherActor))
  (bind _output_get (set `self.BP PlayerPawnRef` _asbp_third_person_pawn))
  (`/Game/ProjectTD/Blueprints/Player/BP_ThirdPerson_Pawn.AddInteractable` _output_get self))

(event `self.Sensor.OnComponentEndOverlap`
  (params (OverlappedComponent :type "PrimitiveComponent Object Reference") (OtherActor :type "Actor Object Reference") (OtherComp :type "PrimitiveComponent Object Reference") (OtherBodyIndex :type Integer))
  (bind _asbp_third_person_pawn (cast `/Game/ProjectTD/Blueprints/Player/BP_ThirdPerson_Pawn` OtherActor))
  (set `self.BP PlayerPawnRef` null)
  (`/Game/ProjectTD/Blueprints/Player/BP_ThirdPerson_Pawn.RemoveInteractable` _asbp_third_person_pawn self))

(event `/Game/ProjectTD/3DAssets/Building/BPI_Interactable.交互开始`
  (params (Instigator :type "Actor Object Reference"))
  (bind (_quantityadded _returnvalue) (`TDInventoryBlueprintLibrary.TryAddItem` Instigator (`self.ItemID`) (`self.Quantity`)))
  (if _returnvalue
    (`self.K2_DestroyActor`)
    (else
      (`KismetSystemLibrary.PrintString` "背包满了"))))

(event `/Game/ProjectTD/3DAssets/Building/BPI_Interactable.与物体开始接触`
  (params (Instigator :type "Actor Object Reference"))
  (`SceneComponent.SetVisibility` (`self.InteractWidget`) true false))

(event `/Game/ProjectTD/3DAssets/Building/BPI_Interactable.与物体结束接触`
  (params (Instigator :type "Actor Object Reference"))
  (`SceneComponent.SetVisibility` (`self.InteractWidget`) false false))

(fn `UserConstructionScript`)

(fn `创建交互UI控件`
  (cast `/Game/UI/UMG/Common/WBP_ItemInteract` (`WidgetComponent.GetUserWidgetObject` (`self.InteractWidget`))))

(fn `初始化`
  (bind _returnvalue (`|GetDataTableRow` "/Game/ProjectTD_Old/DataStructure/DT_Item.DT_Item" (`self.ItemID`))
    (:`then`
      (bind (_displayname _description _icon _itemtype _bisstackable _maxstacksize _dropmesh) (break `/Game/ProjectTD_Old/DataStructure/F_ItemData` _returnvalue))
      (`StaticMeshComponent.SetStaticMesh` (`self.StaticMesh`) _dropmesh)
      (set `self.ItemName` _displayname))))

(fn `获取交互物品信息`
  (returns (InteractItemName :type Text) (Quantity :type Integer))
  (return (`self.ItemName`) (`self.Quantity`)))

(fn `获取消耗材料数组`
  (returns (UpgradeCostArray :type "Array of /Game/ProjectTD_Old/DataStructure/F_CostItem Structure"))
  (return))