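; AC_Equipment is an actor component that tracks which items its owner has equipped, in a map keyed by equipment slot.
; On BeginPlay it caches the owner's AC_Inventory component.
; Equipping reads an inventory slot, checks its DT_Item row against the target slot and stores it if that slot is free.
; If occupied, it only calls unequip with a fixed enum value, which removes that map entry.
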(event `self.ReceiveBeginPlay`
  (`self.初始化`))

(fn `初始化`
  (bind _returnvalue (`self.GetOwner`))
  (`/Engine/EditorBlueprintResources/StandardMacros.IsValid` _returnvalue
    (:`Is Valid`
      (set `self.AC_InventoryRef` (`Actor.GetComponentByClass` _returnvalue "/Game/ProjectTD/Blueprints/ActorComponent/AC_Inventory.AC_Inventory_C")))
    (:`Is Not Valid`
      (`KismetSystemLibrary.PrintString` "错误：未找到背包组件！"))))

(fn `取消装备物品`
  (params (TargetSlot :type "/Game/ProjectTD/结构与枚举/E_EquipmentSlot Enum" :default "NewEnumerator0"))
  (bind _returnvalue (`BlueprintMapLibrary.Map_Remove` (`self.EquipSlots`) TargetSlot))
  (if _returnvalue
    _))

(fn `装备物品`
  (params (InventoryIndex :type Integer) (TargetSlot :type "/Game/ProjectTD/结构与枚举/E_EquipmentSlot Enum" :default "NewEnumerator0"))
  (locals (EquipSlot :type "/Game/ProjectTD/结构与枚举/F_InventorySlot Structure"))
  (bind _output_get (set `local.EquipSlot` (`|GetArrayItem` (`/Game/ProjectTD/Blueprints/ActorComponent/AC_Inventory.Slots` (`self.AC_InventoryRef`)) InventoryIndex)))
  (bind _returnvalue (`|GetDataTableRow` "/Game/ProjectTD/结构与枚举/DT_Item.DT_Item" (`.ItemID_2_7C14D0294170F80B475BA5B300848896` (break `/Game/ProjectTD/结构与枚举/F_InventorySlot` _output_get)))
    (:`then`
      (if (`|EnumEquality` (`.EquipSlot_60_A382031D4D5AC10786F1FCA58952ACBC` (break `/Game/ProjectTD/结构与枚举/F_ItemData` _returnvalue)) TargetSlot)
        (if (`.ReturnValue` (`BlueprintMapLibrary.Map_Find` (`self.EquipSlots`) TargetSlot))
          (`self.取消装备物品` "NewEnumerator0")
          (else
            (`BlueprintMapLibrary.Map_Add` (`self.EquipSlots`) TargetSlot (`local.EquipSlot`))))
        (else
          (return))))))