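; Base building actor that starts from a DT_BuildingTable row and can be repaired by the player through an interaction prompt.
; While the building is level 0, a timeline drives the repair progress bar, reversing when repair stops or interaction ends.
; A completed repair loads the row's NextLevelID data, swaps the mesh and replaces the repair widget with the WBP_OpenMenu widget created at initialization.
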(event `self.ReceiveBeginPlay`
  (`self.初始化`))

(event `/Game/ProjectTD/Blueprints/Building/BPI_Interactable.主角蓝图引用`
  (params (Player :type "/Game/ProjectTD/Blueprints/BP_PlayerCharacter Object Reference"))
  (if (`self.IsBroken`)
    _))

(event `/Game/ProjectTD/Blueprints/Building/BPI_Interactable.与物体开始交互`
  (`self.显示交互信息`))

(event `/Game/ProjectTD/Blueprints/Building/BPI_Interactable.与物体结束交互`
  (`|ExecutionSequence`
    (:`then_0`
      (`self.隐藏交互信息`))
    (:`then_1`
      (if (== (`.LevelIndex_29_C550ADC6402E3763AF5920B3CEDDD6B6` (break `/Game/ProjectTD/结构与枚举/F_BuildingConfig` (`self.CachedBuildingData`))) 0) :!label _label
        (bind (_direction _alpha) (`Timeline|RepairBrokenBuilding` :!via `Reverse` :!label _label_2)
          (:`Update`
            (set `/Game/UI/WBP_RepairWidget.PBarPercent` _alpha (`self.RepairWidget`)))
          (:`Finished`
            (switch `ETimelineDirection` _direction
              (:`Forward`
                (`self.升级建筑`)
                (`self.更新交互面板`)))))))))

(event `/Game/ProjectTD/Blueprints/Building/BPI_Interactable.开始修复建筑`
  (if (== (`.LevelIndex_29_C550ADC6402E3763AF5920B3CEDDD6B6` (break `/Game/ProjectTD/结构与枚举/F_BuildingConfig` (`self.CachedBuildingData`))) 0)
    (goto _label_2 :!via `PlayFromStart`)))

(event `/Game/ProjectTD/Blueprints/Building/BPI_Interactable.停止修复建筑`
  (goto _label))

(fn `UserConstructionScript`)

(fn `初始化`
  (bind _returnvalue (`|GetDataTableRow` "/Game/ProjectTD/结构与枚举/DT_BuildingTable.DT_BuildingTable" (`self.CurrentRowID`))
    (:`then`
      (set `self.CachedBuildingData` _returnvalue)
      (`self.更换模型`)
      ;[1 1 1] UI
      (bind _aswbp_repair_widget (cast `/Game/UI/WBP_RepairWidget` (`WidgetComponent.GetUserWidgetObject` (`self.PromptWidget`))))
      (set `self.RepairWidget` _aswbp_repair_widget)
      (bind _returnvalue_2 (`|CreateWidget` "/Game/UI/WBP_OpenMenu.WBP_OpenMenu_C" (`GameplayStatics.GetPlayerController` 0))) ; 必须有这一步，不然给PromptWidget赋值会出错，因为CommonUI要指定playercontroller
      (set `self.OpenWidget` _returnvalue_2)
      (return))
    (:`RowNotFound`
      (`KismetSystemLibrary.PrintString` "未找到建筑ID"))))

(fn `升级建筑`
  ;[1 1 1] 设置建筑升级后的数据（下一个数据）
  (bind _output_get (set `self.CurrentRowID` (`.NextLevelID_35_82916F394C932E8854C8F8AC5171E11E` (break `/Game/ProjectTD/结构与枚举/F_BuildingConfig` (`self.CachedBuildingData`)))))
  (bind _returnvalue (`|GetDataTableRow` "/Game/ProjectTD/结构与枚举/DT_BuildingTable.DT_BuildingTable" _output_get)
    (:`then`
      (set `self.CachedBuildingData` _returnvalue)
      (set `self.CurrentLevel` 1)
      (`self.更换模型`))))

(fn `显示交互信息`
  (`SceneComponent.SetVisibility` (`self.PromptWidget`) true false))

(fn `更换模型`
  (`StaticMeshComponent.SetStaticMesh` (`self.StaticMesh`) (`.BuildingMesh_47_1015877B49C5652C35B6089BBE56A7AC` (break `/Game/ProjectTD/结构与枚举/F_BuildingConfig` (`self.CachedBuildingData`))))
  (return))

(fn `更新交互面板`
  (bind _openwidget (`self.OpenWidget`))
  (`WidgetComponent.SetWidget` (`self.PromptWidget`) _openwidget)
  (`KismetSystemLibrary.PrintString` (`KismetSystemLibrary.GetDisplayName` _openwidget)))

(fn `获取消耗材料数组`
  (returns (UpgradeCostArray :type "Array of /Game/ProjectTD/结构与枚举/F_BuildCostItem Structure"))
  (return (`.UpgradeCost_49_58FC28D3433E71B7F29DCCB07C878B54` (break `/Game/ProjectTD/结构与枚举/F_BuildingConfig` (`self.CachedBuildingData`)))))

(fn `隐藏交互信息`
  (`SceneComponent.SetVisibility` (`self.PromptWidget`) false false))