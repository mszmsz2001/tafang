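; Health component that gives its owning actor damage, death, healing and optional auto-regeneration.
; It binds to the owner's OnTakeAnyDamage, reduces Health, reports the hit to the instigator and starts a delayed looping timer that restores one point per tick.
; OnRep_Health fires OnDying and reports the kill when health is depleted.
; AddHealth writes clamped health only on authority, and InstantKill applies current health as damage.
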(event `self.ReceiveBeginPlay`
  (bind _output_get (set `self.Owner Actor` (`self.GetOwner`)))
  (add `Actor.OnTakeAnyDamage` _output_get (delegate `TakingDamage`)))

(event `TakingDamage`
  (params (DamagedActor :type "Actor Object Reference") (Damage :type "Float (single-precision)") (DamageType :type "DamageType Object Reference") (InstigatedBy :type "Controller Object Reference") (DamageCauser :type "Actor Object Reference"))
  ; The Taking Damage event is always triggered when the actor that owns this component takes any damage.
  (`self.Take Damage` Damage InstigatedBy DamageCauser) ; Apply damage
)

(event `Start Health Recover`
  ; The Taking Damage event is always triggered when the actor that owns this component takes any damage.
  (bind _returnvalue (`KismetSystemLibrary.K2_SetTimer` null "Health Revocer Cycle" (`self.Recover Speed`) true false (`self.Auto Recover Start Delay`)))
  (set `self.Auto Recover Timer` _returnvalue))

(fn `Add Health`
  (params (`Health Amount To Add` :type "Float (double-precision)"))
  (returns (`Return Added Amount` :type "Float (double-precision)"))
  (locals (`Previouse Health Points` :type "Float (double-precision)" :default 0.0) (`New Health Points` :type "Float (double-precision)" :default 0.0) (`Added Amount` :type "Float (double-precision)"))
  (set `local.Previouse Health Points` (`self.Health`) :!pinned true) ; Saves the previous amount of health points\nbefore adding more health points.
  ; Combine Health Points with Amount to Add
  (set `local.New Health Points` (`KismetMathLibrary.FClamp` (+ (`self.Health`) (`KismetMathLibrary.FMax` (`local.Health Amount To Add`))) 0.0 (`self.Max Health`)))
  (`|ExecutionSequence`
    (:`then_0`
      (`/Engine/EditorBlueprintResources/ActorComponentMacros.Switch Has Authority`
        (:`Authority`
          (set `self.Health` (`local.New Health Points`) :!pinned true) ; Update health points (Run only on the server side)
        )))
    (:`then_1`
      ; Returns added health points amount
      (bind _output_get (set `local.Added Amount` (- (`local.New Health Points`) (`local.Previouse Health Points`))))
      (`self.On Health Points Added` _output_get)
      (return (`local.Added Amount`)))))

(fn `Get Health Ratio`
  (returns (ReturnValue :type "Float (double-precision)"))
  (return (/ (`self.Health`) (`self.Max Health`))))

(fn `Health Is Full`
  (returns (ReturnValue :type Boolean))
  (return (>= (`self.Health`) (`self.Max Health`))))

(fn `Health Revocer Cycle`
  (if (and (`self.Eanble Auto Recover`) (`self.Is Alive`) (not (`self.Health Is Full`)))
    (`/Engine/EditorBlueprintResources/StandardMacros.IncrementFloat` (`self.Health`) :!pinned true) ; adds 1 health point at each auto recover cycle
    (else
      (`KismetSystemLibrary.K2_ClearAndInvalidateTimerHandle` (`self.Auto Recover Timer`) :!pinned true) ; Stops the health recover cycle
    )))

(fn `Instant Kill`
  (params (Killer :type "Actor Object Reference") (`Kill Instigator` :type "Controller Object Reference"))
  (`GameplayStatics.ApplyDamage` (`self.Owner Actor`) (`self.Health`) (`local.Kill Instigator`) (`local.Killer`)))

(fn `Is Alive`
  (returns (ReturnValue :type Boolean))
  (return (> (`self.Health`) 0.0)))

(fn `OnRep_Health`
  (if (not (> (`self.Health`) 0.0)) :!pinned true
    (`self.On Dying` (`self.Last Damage Instigator`) (`self.Last Damage Causer`) :!pinned true) ; Calls "On Dying" Dispatcher Event that can be used by the owner actor
    (message `/Game/VisualSandbox/Blueprints/Interfaces/BPI_Useful.Report Kill` (`self.Last Damage Instigator`) (`self.GetOwner`))))

(fn `Take Damage`
  (params (Damage :type "Float (double-precision)") (`Damage Instigator` :type "Controller Object Reference") (`Damage Causer` :type "Actor Object Reference"))
  (set `self.Last Damage Instigator` `Damage Instigator`)
  (set `self.Last Damage Causer` `Damage Causer`)
  (if (and (> (`local.Damage`) 0.0) (`self.Is Alive`) (`self.Can Be Damaged`))
    ; Subtracts Health Points
    (set `self.Health` (`KismetMathLibrary.FMax` (- (`self.Health`) (`local.Damage`))))
    (`self.Start Health Recover`)
    (message `/Game/VisualSandbox/Blueprints/Interfaces/BPI_Useful.Report Hit Damage` (`local.Damage Instigator`) (`self.GetOwner`))))