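; AC_Interaction is an interaction component that periodically updates which interactable its owning actor is currently targeting.
; RefreshInteractionTimer runs a looping timer only while OverlappingInteractables is non-empty, avoiding per-frame Tick.
; Each timer pass calls UpdateCurrentInteractTarget with the component as context and the owner as interactor, or stops the timer if the owner is invalid.
; Target selection and overlap list maintenance happen outside these graphs.
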(fn `RefreshInteractionTimer`
  (if (> (`KismetArrayLibrary.Array_Length` (`self.OverlappingInteractables`)) 0)
    (`self.StartInteractionUpdateTimer`)
    (else
      (`self.StopInteractionUpdateTimer`))))

(fn `StartInteractionUpdateTimer`
  (if (not (`KismetSystemLibrary.K2_IsTimerActiveHandle` (`self.InteractionUpdateTimerHandle`)))
    (`KismetSystemLibrary.K2_SetTimer` null "UpdateInteractTarget_Timer" (`self.InteractionUpdateInterval`) true)))

(fn `StopInteractionUpdateTimer`
  (`KismetSystemLibrary.K2_ClearAndInvalidateTimerHandle` (`self.InteractionUpdateTimerHandle`)))

(fn `UpdateInteractTarget_Timer`
  (bind _returnvalue (`self.GetOwner`))
  (`/Engine/EditorBlueprintResources/StandardMacros.IsValid` _returnvalue
    (:`Is Valid`
      (`TDInteractionBlueprintLibrary.UpdateCurrentInteractTarget` self _returnvalue))
    (:`Is Not Valid`
      (`self.StopInteractionUpdateTimer`))))