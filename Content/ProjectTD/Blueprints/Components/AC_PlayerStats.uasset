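; Player stats component that pushes the player's health and magic values to the HUD widget.
; A single update function passes current and maximum values, plus bar fill ratios, to WBPHUD; BeginPlay and Tick are empty.
; The magic calls appear swapped: the current MP readout receives the ratio and the MP bar receives the raw current value.
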(fn `更新HUD玩家信息`
  (bind _wbp_hud (`self.WBP_HUD`))
  (message `/Game/UI/Interface/BI_HPMP.UpdatePlayerCurrentHP` _wbp_hud (`self.CurrentHealth`))
  (message `/Game/UI/Interface/BI_HPMP.UpdatePlayerHPBarPercent` _wbp_hud (/ (`self.CurrentHealth`) (`self.MaxHealth`)))
  (message `/Game/UI/Interface/BI_HPMP.UpdatePlayerMaxHP` _wbp_hud (`self.MaxHealth`))
  (message `/Game/UI/Interface/BI_HPMP.UpdatePlayerMaxMP` _wbp_hud (`self.MaxMagic`))
  (message `/Game/UI/Interface/BI_HPMP.UpdatePlayerCurrentMP` _wbp_hud (/ (`self.CurrentMagic`) (`self.MaxMagic`)))
  (message `/Game/UI/Interface/BI_HPMP.UpdatePlayerMPBarPercent` _wbp_hud (`self.CurrentMagic`)))