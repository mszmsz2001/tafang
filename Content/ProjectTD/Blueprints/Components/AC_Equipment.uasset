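; AC_Equipment is an actor component that manages equipped items per slot and creates the WBP_Equipment widget on BeginPlay.
; Equipping looks up an AC_Inventory item in DT_Item and requires a matching slot type.
; It moves the item into the EquipSlots map, swapping any worn item back into that inventory cell, then broadcasts OnEquipmentUpdate and refreshes inventory UI.
; Unequipping only removes the map entry, without returning the item or broadcasting.
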(event `self.ReceiveBeginPlay`
  (`self.初始化`))

(fn `初始化`
  (bind _returnvalue (`self.GetOwner`))
  (`/Engine/EditorBlueprintResources/StandardMacros.IsValid` _returnvalue
    (:`Is Valid`
      (set `self.AC_InventoryRef` (`Actor.GetComponentByClass` _returnvalue "/Game/ProjectTD/Blueprints/Components/AC_Inventory.AC_Inventory_C"))
      (`|CreateWidget` "/Game/UI/WBP_Equipment.WBP_Equipment_C" (`GameplayStatics.GetPlayerController` 0) self))
    (:`Is Not Valid`
      (`KismetSystemLibrary.PrintString` "错误：未找到背包组件！"))))

(fn `卸下装备物品`
  (params (TargetSlot :type "/Game/ProjectTD_Old/DataStructure/E_EquipmentSlot Enum" :default "NewEnumerator0"))
  (bind _returnvalue (`BlueprintMapLibrary.Map_Remove` (`self.EquipSlots`) TargetSlot))
  (if _returnvalue
    _))

(fn `更新装备信息`
  (`self.OnEquipmentUpdate`)
  (return))

(fn `装备物品`
  (params (InventoryIndex :type Integer) (TargetSlot :type "/Game/ProjectTD_Old/DataStructure/E_EquipmentSlot Enum" :default "NewEnumerator0"))
  (locals (EquipSlot :type "/Game/ProjectTD_Old/DataStructure/F_InventorySlot Structure") (EquipType :type "/Game/ProjectTD_Old/DataStructure/E_EquipmentSlot Enum"))
  (bind (_value _returnvalue) (`BlueprintMapLibrary.Map_Find` (`self.EquipSlots`) TargetSlot))
  (bind _output_get (set `local.EquipSlot` (`|GetArrayItem` (`/Game/ProjectTD/Blueprints/Components/AC_Inventory.Slots` (`self.AC_InventoryRef`)) InventoryIndex)))
  (bind _returnvalue_2 (`|GetDataTableRow` "/Game/ProjectTD_Old/DataStructure/DT_Item.DT_Item" (`.ItemID_2_7C14D0294170F80B475BA5B300848896` (break `/Game/ProjectTD_Old/DataStructure/F_InventorySlot` _output_get)))
    (:`then`
      (bind (_displayname _description _icon _itemtype _bisstackable _maxstacksize _dropmesh _equipslot) (break `/Game/ProjectTD_Old/DataStructure/F_ItemData` _returnvalue_2))
      (set `local.EquipType` _equipslot)
      (if (`|EnumEquality` _equipslot TargetSlot)
        (if _returnvalue
          (`/Game/ProjectTD/Blueprints/Components/AC_Inventory.替换某格物品` (`self.AC_InventoryRef`) (`local.InventoryIndex`) _value)
          (`BlueprintMapLibrary.Map_Add` (`self.EquipSlots`) (`local.EquipType`) (`local.EquipSlot`))
          (`self.更新装备信息`)
          (`/Game/ProjectTD/Blueprints/Components/AC_Inventory.刷新背包物品(UI)` (`self.AC_InventoryRef`))
          (else
            (`BlueprintMapLibrary.Map_Add` (`self.EquipSlots`) TargetSlot (`local.EquipSlot`))
            (`/Game/ProjectTD/Blueprints/Components/AC_Inventory.移除某格物品` (`self.AC_InventoryRef`) (`local.InventoryIndex`))
            (`self.更新装备信息`)
            (`/Game/ProjectTD/Blueprints/Components/AC_Inventory.刷新背包物品(UI)` (`self.AC_InventoryRef`))))
        (else
          (return))))))