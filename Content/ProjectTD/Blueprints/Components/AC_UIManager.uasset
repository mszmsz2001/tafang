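; AC_UIManager is an actor component that opens and closes UI widgets, including the tower defense build menu.
; On BeginPlay it caches the first player controller as BP_MyPlayerController.
; OpenMenu creates a widget of the given class, stores it, adds it to the viewport and optionally shows the mouse cursor.
; OpenBuildMenu wraps OpenMenu with the build menu class, and CloseMenu removes the last stored widget.
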(event `self.ReceiveBeginPlay`
  (bind _asbp_my_player_controller (cast `/Game/ProjectTD_Old/Blueprints/BP_MyPlayerController` (`GameplayStatics.GetPlayerController` 0)))
  (set `self.My PlayerController` _asbp_my_player_controller))

(fn `CloseMenu`
  (`Widget.RemoveFromParent` (`self.TargetWidget`)))

(fn `OpenBuildMenu`
  (params (ShowCursor :type Boolean))
  (`self.OpenMenu` (`self.WBP_BuildMenu`) ShowCursor))

(fn `OpenMenu`
  (params (ObjectWidget :type "UserWidget Class Reference") (ShowCursor :type Boolean))
  (bind _returnvalue (`|CreateWidget` ObjectWidget))
  (bind _output_get (set `self.TargetWidget` _returnvalue))
  (`UserWidget.AddToViewport` _output_get 0)
  (if ShowCursor
    (set `PlayerController.bShowMouseCursor` true (`self.My PlayerController`))))