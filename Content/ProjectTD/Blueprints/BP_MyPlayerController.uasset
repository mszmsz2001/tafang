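; BP_MyPlayerController is the player controller that routes Enhanced Input to the player pawn and build menu.
; BeginPlay adds the IMC_Default mapping context, and possession caches the pawn as BP_MyPlayer.
; IA_Move forwards WASD movement to the pawn's HandleMove.
; IA_Build (B) toggles the build menu through ACUIManager using the HasBuildMenu flag, while IA_Click is an empty stub.
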(event `self.ReceiveBeginPlay`
  (bind _returnvalue (subsystem `EnhancedInputLocalPlayerSubsystem`))
  ; 添加输入上下文映射
  (`/Engine/EditorBlueprintResources/StandardMacros.IsValid` _returnvalue
    (:`Is Valid`
      (`EnhancedInputSubsystemInterface.AddMappingContext` _returnvalue "/Game/ProjectTD/Input/IMC_Default.IMC_Default" 0 (struct)))))

(event `EnhancedInput|/Game/ProjectTD/Input/Actions/IA_Move`
  (params (ActionValue :type "Vector2D Structure") (ElapsedSeconds :type "Float (double-precision)") (TriggeredSeconds :type "Float (double-precision)") (InputAction :type "InputAction Object Reference" :default "/Game/ProjectTD/Input/Actions/IA_Move.IA_Move"))
  ; 角色移动 WASD
  (:`Triggered`
    (`/Game/ProjectTD/Blueprints/BP_MyPlayer.HandleMove` (`self.Controlled Pawn`) ActionValue)))

(event `EnhancedInput|/Game/ProjectTD/Input/Actions/IA_Click`
  (params (ActionValue :type Boolean) (ElapsedSeconds :type "Float (double-precision)") (TriggeredSeconds :type "Float (double-precision)") (InputAction :type "InputAction Object Reference" :default "/Game/ProjectTD/Input/Actions/IA_Click.IA_Click")))

(event `EnhancedInput|/Game/ProjectTD/Input/Actions/IA_Build`
  (params (ActionValue :type Boolean) (ElapsedSeconds :type "Float (double-precision)") (TriggeredSeconds :type "Float (double-precision)") (InputAction :type "InputAction Object Reference" :default "/Game/ProjectTD/Input/Actions/IA_Build.IA_Build"))
  (bind _ac_uimanager (`self.AC_UIManager`))
  ; 打开/关闭 建造菜单[B]
  (:`Started`
    (if (`self.HasBuildMenu`)
      (`/Game/ProjectTD/Blueprints/ActorComponent/AC_UIManager.CloseMenu` _ac_uimanager)
      (set `self.HasBuildMenu` false)
      (else
        (`/Game/ProjectTD/Blueprints/ActorComponent/AC_UIManager.OpenBuildMenu` _ac_uimanager true)
        (set `self.HasBuildMenu` true)))))

(event `self.ReceivePossess`
  (params (PossessedPawn :type "Pawn Object Reference"))
  (bind _asbp_my_player (cast `/Game/ProjectTD/Blueprints/BP_MyPlayer` PossessedPawn))
  (set `self.Controlled Pawn` _asbp_my_player))

(fn `UserConstructionScript`)