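; Behavior tree task that makes an AI shooter fire its equipped firearm for a set number of shots, failing if it holds no firearm.
; It sets the firearm's shot alignment mode, then counts shots through the OnShotsFired event and a resettable DoN, finishing successfully at the limit.
; Non-automatic weapons release the trigger after each shot and re-fire on a timer slightly longer than the fire interval.
; Abort stops shooting and clears that timer.
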(event `self.ReceiveExecuteAI`
  (params (OwnerController :type "AIController Object Reference") (ControlledPawn :type "Pawn Object Reference"))
  (`parent.ReceiveExecuteAI` OwnerController ControlledPawn)
  (`self.Restart Counter`)
  (bind _asbp_firearm (cast `/Game/VisualSandbox/Blueprints/Weapons/Firearms/BP_Firearm` (`/Game/VisualSandbox/Blueprints/Characters/BP_ShooterCharacter.Character Equipment` (`self.ShooterPawn`)))
    (:`then`
      (bind _output_get (set `self.Firearm` _asbp_firearm))
      (set `/Game/VisualSandbox/Blueprints/Weapons/Firearms/BP_Firearm.Shot Alignment Mode` "NewEnumerator1" _output_get)
      (add `/Game/VisualSandbox/Blueprints/Weapons/Firearms/BP_Firearm.OnShotsFired` (`self.Firearm`) (delegate `Count Each Shots`))
      (`self.Start Shooting`))
    (:`CastFailed`
      (`self.FinishExecute` false))))

(event `Count Each Shots`
  ; Shots counter
  (if (not (`/Game/VisualSandbox/Blueprints/Weapons/Firearms/BP_Firearm.Fully Automatic` (`self.Firearm`)))
    (`self.Stop Shooting`))
  (bind _counter (`/Engine/EditorBlueprintResources/StandardMacros.Do N` (`self.Number Of Shots`) :!label _label)
    (:`Exit`
      (if (>= _counter (`self.Number Of Shots`))
        (`self.Stop Shooting`)
        (`self.FinishExecute` true)
        (elif (not (`/Game/VisualSandbox/Blueprints/Weapons/Firearms/BP_Firearm.Fully Automatic` (`self.Firearm`)))
          (bind _returnvalue (`KismetSystemLibrary.K2_SetTimer` null "Start Shooting" (+ (`/Game/VisualSandbox/Blueprints/Weapons/Firearms/BP_Firearm.Get Fire Interval` (`self.Firearm`)) 0.25)))
          (set `self.Shooting Timer` _returnvalue))))))

(event `Restart Counter`
  ; Shots counter
  (goto _label :!via `Reset`))

(event `self.ReceiveAbortAI`
  (params (OwnerController :type "AIController Object Reference") (ControlledPawn :type "Pawn Object Reference"))
  ; Aborting
  (`self.Stop Shooting`)
  (`KismetSystemLibrary.K2_ClearAndInvalidateTimerHandle` (`self.Shooting Timer`))
  (`self.FinishAbort`))

(event `Start Shooting`
  ; Start / Stop Shooting
  (`/Game/VisualSandbox/Blueprints/Characters/BP_ShooterCharacter.Start Shooting` (`self.ShooterPawn`) true))

(event `Stop Shooting`
  ; Start / Stop Shooting
  (`/Game/VisualSandbox/Blueprints/Characters/BP_ShooterCharacter.Start Shooting` (`self.ShooterPawn`) false))