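; Behavior tree task for the sentry gun AI that waits until the turret is aimed at its target.
; Each tick it line traces on the Camera channel from the pawn's eye view point along the turret rotation's forward vector, ignoring the pawn itself.
; It finishes successfully once the hit actor matches the Target blackboard value, and has no failure path of its own.
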(event `self.ReceiveTickAI`
  (params (OwnerController :type "AIController Object Reference") (ControlledPawn :type "Pawn Object Reference") (DeltaSeconds :type "Float (single-precision)"))
  (bind _sentrygunpawn (`self.SentryGunPawn`))
  (bind _outlocation (`Actor.GetActorEyesViewPoint` _sentrygunpawn))
  (bind _outhit (`KismetSystemLibrary.LineTraceSingle` _outlocation (+ _outlocation (* (`KismetMathLibrary.GetForwardVector` (`/Game/VisualSandbox/Blueprints/Weapons/SentryGun/BP_SentryGun.Turret Rotation` _sentrygunpawn)) 10000.0)) "TraceTypeQuery2" false (`|MakeArray` (`self.SentryGunPawn`) :!type "Actor Object Reference")))
  (if (== (`.HitActor` (`GameplayStatics.BreakHitResult` _outhit)) (`BTFunctionLibrary.GetBlackboardValueAsActor` (`self.Target`)))
    (`self.FinishExecute` true)))