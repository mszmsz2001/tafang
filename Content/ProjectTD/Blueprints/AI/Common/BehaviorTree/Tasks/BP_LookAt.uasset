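; Behavior tree task that turns an AI controller's focus toward the Target blackboard key.
; On its AI tick, it focuses on the key's actor if valid, otherwise uses the key's vector as a focal point, then finishes successfully.
; The focus stays set after completion and is cleared only when the task is aborted.
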(event `self.ReceiveTickAI`
  (params (OwnerController :type "AIController Object Reference") (ControlledPawn :type "Pawn Object Reference") (DeltaSeconds :type "Float (single-precision)"))
  (set `self.Pawn Controller` OwnerController)
  (`|ExecutionSequence`
    (:`then_0`
      (bind _output_get (set `self.Target Pawn` (`BTFunctionLibrary.GetBlackboardValueAsActor` (`self.Target`))))
      (`/Engine/EditorBlueprintResources/StandardMacros.IsValid` _output_get
        (:`Is Valid`
          (`AIController.K2_SetFocus` (`self.Pawn Controller`) (`self.Target Pawn`)))
        (:`Is Not Valid`
          (`AIController.K2_SetFocalPoint` (`self.Pawn Controller`) (`BTFunctionLibrary.GetBlackboardValueAsVector` (`self.Target`))))))
    (:`then_1`
      (`self.FinishExecute` true))))

(event `self.ReceiveAbortAI`
  (params (OwnerController :type "AIController Object Reference") (ControlledPawn :type "Pawn Object Reference"))
  (`AIController.K2_ClearFocus` OwnerController))